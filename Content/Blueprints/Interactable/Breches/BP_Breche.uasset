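; BP_Breche is an interactable breach that the player clears by bringing it wood and rope pickups.
; The construction script randomizes how many of each it needs, and two text renders refresh those remaining counts every Tick.
; When a third-person character carrying either item overlaps the box, the matching count drops and the item is dropped and destroyed.
; Assemblage then destroys the breach once both counts reach zero.
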(event OnComponentBeginOverlap(Box)
  (params (OverlappedComponent :type Primitive%20Component%20Object%20Reference) (OtherActor :type Actor%20Object%20Reference) (OtherComp :type Primitive%20Component%20Object%20Reference) (OtherBodyIndex :type Integer) (bFromSweep :type Boolean) (SweepResult :type Hit%20Result%20Structure%20%28by%20ref%29))
  (bind _asbp_third_person_character (Utilities|Casting|CastToBP_ThirdPersonCharacter OtherActor))
  (if (== (Utilities|GetClass (Variables|/Game/ThirdPerson/Blueprints/BP_ThirdPersonCharacter.BP_ThirdPersonCharacter_C|GetBP_PickUp _asbp_third_person_character)) "/Game/Blueprints/Interactable/BP_PickUp_Wood.BP_PickUp_Wood_C")
    (bind _result (Math|Integer|DecrementInt (Variables|Default|GetNombresBois))
      (:%20%20
        (Variables|Default|SetNombresBois (Math|Integer|Clamp(Integer) _result 0 2))
        (Default|DropItem _asbp_third_person_character :!label _label)
        (Actor|DestroyActor (Variables|/Game/ThirdPerson/Blueprints/BP_ThirdPersonCharacter.BP_ThirdPersonCharacter_C|GetPickedUp%20Item _asbp_third_person_character))
        (CallFunction|Assemblage)))
    (elif (== (Utilities|GetClass (Variables|/Game/ThirdPerson/Blueprints/BP_ThirdPersonCharacter.BP_ThirdPersonCharacter_C|GetBP_PickUp _asbp_third_person_character)) "/Game/Blueprints/Interactable/BP_PickUp_Rope.BP_PickUp_Rope_C")
      (bind _result_2 (Math|Integer|DecrementInt (Variables|Default|GetNombreCordes))
        (:%20%20
          (Variables|Default|SetNombreCordes (Math|Integer|Clamp(Integer) _result_2 0 2))
          (goto _label))))))

(event Custom|Assemblage
  (if (and (== (Variables|Default|GetNombresBois) 0) (== (Variables|Default|GetNombreCordes) 0))
    (Actor|DestroyActor)))

(event EventTick
  (params (DeltaSeconds :type Float%20%28single-precision%29))
  (Rendering|Components|TextRender|SetText (Variables|Default|GetTextRender) (Utilities|Text|ToText(Integer) (Variables|Default|GetNombresBois)))
  (Rendering|Components|TextRender|SetText (Variables|Default|GetTextRender1) (Utilities|Text|ToText(Integer) (Variables|Default|GetNombreCordes))))

(fn ConstructionScript
  (Variables|Default|SetNombreCordes (Math|Random|RandomIntegerinRange 1 2))
  (Variables|Default|SetNombresBois (Math|Random|RandomIntegerinRange 1 2)))