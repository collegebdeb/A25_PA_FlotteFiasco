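; Harpoon pickup that lets the player aim at interactables in the water and reel them in, with an energy boost or penalty.
; UpdateVisee extends a debug-drawn aim forward over time, keeping the overlapped actor nearest its tip, ignoring BP_CollectPoisson.
; TriggerLancer locks the player to the raft and starts a timed joystick prompt.
; Each PullCollectible call lerps the target closer until it switches into the player's hands; timeout or mid-pull drop destroys it.
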(event Custom|TriggerLancer
  (bind _player (Variables|Default|GetPlayer))
  ;[0.15 0.15 0.15 0.5] Si un interactable est touché on peut commencer a sortir le poisson de l'eau
  (if (Variables|Default|GetHitTarget?)
    (Variables|Default|SetHarponnageEnCours true)
    (Pawn|Components|CharacterMovement|DisableMovement (Variables|/Script/Engine.Character|GetCharacterMovement _player))
    (Variables|/Game/ThirdPerson/Blueprints/BP_ThirdPersonCharacter.BP_ThirdPersonCharacter_C|SetdisabledMovement? _player true)
    (Transformation|AttachActorToActor (Variables|Default|GetPlayer) (Variables|Default|GetRaft) "None" "KeepWorld" "KeepWorld" "KeepWorld" true)
    (bind _returnvalue (AddComponent|AddWidgetComponent (Variables|Default|GetItemACollecter) false))
    (bind _output_get (Variables|Default|SetWB_Joystick _returnvalue))
    (Rendering|SetVisibility _output_get true false)
    (bind _returnvalue_2 (Utilities|Time|SetTimerbyEvent (delegate Custom|TimerEnd) 5.0))
    (Variables|Default|SetTimer _returnvalue_2)))

(event Custom|PullCollectible
  ;[0.15 0.15 0.15 0.5] Attire l'interactable de l'eau vers le joueur
  (if (Variables|Default|GetHarponnageEnCours)
    (bind _itemacollecter (Variables|Default|GetItemACollecter)
      (:then
        (Transformation|SetWorldLocation (Variables|/Game/Blueprints/Interactable/Parent/BP_Interactable_PickUp.BP_Interactable_PickUp_C|GetSM _itemacollecter) (Math|Vector|Lerp(Vector) (Transformation|GetWorldLocation (Variables|/Game/Blueprints/Interactable/Parent/BP_Interactable_PickUp.BP_Interactable_PickUp_C|GetSM _itemacollecter)) (Transformation|GetActorLocation (Variables|Default|GetPlayer)) 0.2) false false)
        ;[0.15 0.15 0.15 0.5] Si réussit à attirer l'objet, le fait spawn dans les mains du joueur
        (if (< (Math|Vector|VectorLengthXY (- (Transformation|GetWorldLocation (Variables|/Script/Engine.Character|GetCapsuleComponent (Variables|Default|GetPlayer))) (Transformation|GetWorldLocation (Variables|/Game/Blueprints/Interactable/Parent/BP_Interactable_PickUp.BP_Interactable_PickUp_C|GetSM (Variables|Default|GetItemACollecter))))) (Variables|Default|GetDistanceCollectibleFromPlayer))
          (Variables|Default|SetHarponnageEnCours false)
          (Variables|Default|SetHitTarget? false)
          (Utilities|Time|ClearandInvalidateTimerbyHandle (Variables|Default|GetTimer))
          (CallFunction|EnergyBoostSuccess (Variables|Default|GetEnergyImpact))
          (Rendering|SetVisibility (Variables|Default|GetWB_Joystick) false false)
          (CallFunction|AttachCollectible)))
      (:else))))

(event Custom|AttachCollectible
  (bind _player (Variables|Default|GetPlayer))
  ;[0.15 0.15 0.15 0.5] Attache le collectible au personnage
  (Transformation|DetachFromActor (Variables|Default|GetPlayer) "KeepWorld" "KeepWorld" "KeepWorld")
  (Default|SwitchCollectible _player self _player (Variables|Default|GetItemACollecter)))

(event Custom|TimerEnd
  (bind _wb_joystick (Variables|Default|GetWB_Joystick))
  ;[0.15 0.15 0.15 0.5] Défaite après timer
  (CallFunction|EnergyMalusDefeat (Variables|Default|GetEnergyImpact))
  (Actor|DestroyActor (Variables|Default|GetItemACollecter))
  (Transformation|DetachFromActor (Variables|Default|GetPlayer) "KeepWorld" "KeepWorld" "KeepWorld")
  (Pawn|Components|CharacterMovement|SetMovementMode (Variables|/Script/Engine.Character|GetCharacterMovement (Variables|Default|GetPlayer)) "MOVE_Walking" 0)
  (Variables|Default|SetHarponnageEnCours false)
  (Variables|Default|SetHitTarget? false)
  (Utilities|Time|ClearandInvalidateTimerbyHandle (Variables|Default|GetTimer))
  (Utilities|IsValid _wb_joystick
    (:Is%20Valid
      (Rendering|SetVisibility _wb_joystick false false))))

(event EventDrop
  (params (Player :type BP%20Third%20Person%20Character%20Object%20Reference))
  ;[0.15 0.15 0.15 0.5] Drop - Parent + reset les variables et détache le joueur du radeau
  (if (Variables|Default|GetHarponnageEnCours)
    (CallFunction|TimerEnd))
  (|CallParentFunction Player)
  (Variables|Default|SetHitTarget? false)
  (Variables|Default|SetHarponnageEnCours false))

(event Collision|EventActorBeginOverlap
  (params (OtherActor :type Actor%20Object%20Reference))
  (|CallParentFunction OtherActor))

(event EventTick
  (params (DeltaSeconds :type Float%20%28single-precision%29))
  (|CallParentFunction DeltaSeconds))

(event Collision|EventActorEndOverlap
  (params (OtherActor :type Actor%20Object%20Reference))
  (|CallParentFunction OtherActor))

(event EventPickUp
  (params (Player :type BP%20Third%20Person%20Character%20Object%20Reference))
  ;[0.15 0.15 0.15 0.5] Pick up - Parent
  (|CallParentFunction Player))

(event EventBeginPlay
  (|CallParentFunction))

(fn ConstructionScript
  (|CallParentFunction))

(fn ActorstoIgnore
  (bind _outactors (Actor|GetAllActorsOfClass "/Game/Blueprints/Stations/Peche/BP_CollectPoisson.BP_CollectPoisson_C"))
  (for _array_element _outactors
    (Utilities|Array|Add (LocalVariables|GetLocalActorsToIgnore) _array_element))
  (bind _output_get (Variables|Default|SetActors%20to%20Ignore (LocalVariables|GetLocalActorsToIgnore)))
  (return _output_get))

(fn UpdateVisee
  (params (ElapsedSeconds :type Float%20%28double-precision%29))
  (bind _player (Variables|Default|GetPlayer))
  (bind _capsulecomponent (Variables|/Script/Engine.Character|GetCapsuleComponent _player))
  (bind _returnvalue (Transformation|GetWorldLocation _capsulecomponent))
  ;[0.15 0.15 0.15 0.5] Fait apparaître une flèche qui va faire la visée. Si la visée touche un acteur alors cela lance une for each loop
  (bind _output_get (LocalVariables|SetPointe (+ (* (Math|Float|Min(Float) (* ElapsedSeconds 3e+02) 9e+02) (Math|Vector|GetForwardVector _capsulecomponent)) _returnvalue)))
  (Rendering|Debug|DrawDebugArrow _returnvalue _output_get 1e+02 "(R=1.000000,G=0.007298,B=0.095167,A=1.000000)" 0.0 1e+01)
  (bind _actorstoignore (CallFunction|ActorstoIgnore))
  (bind _outactors (Collision|CapsuleOverlapActors (LocalVariables|GetPointe) 3e+02 1e+02 (Utilities|Array|MakeArray "ObjectTypeQuery8") 0 _actorstoignore))
  (Rendering|Debug|DrawDebugCapsule (LocalVariables|GetPointe) 3e+02 1e+02 "0, 0, 0" "(R=1.000000,G=1.000000,B=1.000000,A=1.000000)" 0.0 1e+01)
  (for (_array_element _array_index) _outactors
    ;[0.15 0.15 0.15 0.5] Pour le premier index (actor touché) l'enregistre en variable locale.
    (if (== _array_index 0)
      (LocalVariables|SetHitActor _array_element)
      (LocalVariables|SetdistanceFromPointe (Math|Vector|Distance(Vector) (Transformation|GetActorLocation (LocalVariables|GetHitActor)) (LocalVariables|GetPointe)))
      (else
        ;[0.15 0.15 0.15 0.5] Pour les index suivants (autres acteurs overlappés), cela les compare aux objets frappés précédemment. Si l'objet est plus proche de la pointe de la visée que le précédent cela override la variable locale.
        (if (< (Math|Vector|Distance(Vector) (Transformation|GetActorLocation _array_element) (LocalVariables|GetPointe)) (LocalVariables|GetdistanceFromPointe))
          (LocalVariables|SetdistanceFromPointe (Math|Vector|Distance(Vector) (Transformation|GetActorLocation _array_element) (LocalVariables|GetPointe)))
          (LocalVariables|SetHitActor _array_element)))))
  ;[0.15 0.15 0.15 0.5] A la fin de la loop, prends la variable locale correspondant à l'objet hit et l'enregistre afin de l'utiliser dans l'event graph.
  (bind _asbp_interactable_pick_up (Utilities|Casting|CastToBP_Interactable_PickUp (LocalVariables|GetHitActor)))
  (Variables|Default|SetItemACollecter _asbp_interactable_pick_up)
  (Variables|Default|SetHitTarget? true)
  (CallFunction|HitFeedback (LocalVariables|GetHitActor)))

(fn HitFeedback
  (params (HitActor :type Actor%20Object%20Reference))
  (bind _returnvalue (AddComponent|AddWidgetComponent HitActor false))
  (bind _output_get (Variables|Default|SetWB_Exclamation _returnvalue))
  (Rendering|SetVisibility _output_get true false))