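; Game mode for the mobile raft game, managing UI, minigame selection and raft effects.
; BeginPlay shows the cursor, adds hidden settings and pause widgets, then opens the barrel (Tonneau) widget.
; Helpers open a random minigame from Protector or Saboteur pools, refill energy widgets, and push or spin BP_Raft_Base1 through physics.
; SpawnVagues only iterates Gerstner waves; its editing nodes and several pause-menu tests are disconnected.
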(event Custom|SetWidgets
  (bind _returnvalue (UserInterface|CreateWidget "/Game/Mobile/Widgets/Menus/WB_Mobile_Settings.WB_Mobile_Settings_C"))
  (bind _output_get (Variables|Default|SetWB_Settings _returnvalue))
  (UserInterface|Viewport|AddtoViewport _output_get 0)
  (Widget|SetVisibility _output_get "Hidden")
  (bind _returnvalue_2 (UserInterface|CreateWidget "/Game/Mobile/Widgets/Menus/WB_Mobile_PauseGame.WB_Mobile_PauseGame_C"))
  (bind _output_get_2 (Variables|Default|SetWidgetPauseReference _returnvalue_2))
  (UserInterface|Viewport|AddtoViewport _output_get_2 0)
  (Widget|SetVisibility _output_get_2 "Hidden"))

(event EventBeginPlay
  (Variables|/Script/Engine.PlayerController|SetbShowMouseCursor (Game|GetPlayerController 0) true)
  (CallFunction|SetWidgets)
  (bind _returnvalue (UserInterface|CreateWidget "/Game/Mobile/Widgets/Mini-jeux/WB_Mobile_Tonneau.WB_Mobile_Tonneau_C"))
  (UserInterface|Viewport|AddtoViewport _returnvalue 0))

(event EventTick
  (params (DeltaSeconds :type Float%20%28single-precision%29)))

(fn ConstructionScript)

(fn SpawnVagues
  (bind _outactors (Actor|GetAllActorsOfClass "/Script/Water.WaterBody"))
  (for _array_element _outactors
    (bind _asgerstner_water_waves (Utilities|Casting|CastToGerstnerWaterWaves (Class|WaterBodyComponent|GetWaterWaves (Variables|/Script/Water.WaterBody|GetWaterBodyComponent _array_element))))
    (for _array_element_2 (Variables|/Script/Water.GerstnerWaterWaves|GetGerstnerWaves _asgerstner_water_waves)
      _)))

(fn AddEnergy
  (bind _foundwidgets (Widget|GetAllWidgetsOfClass "/Game/Widgets/EnergyProgressBar/WB_Energy.WB_Energy_C" true))
  (for _array_element _foundwidgets
    (Default|AddEnergy _array_element 3e+01)))

(fn AddImpulseForward
  (bind _returnvalue (Actor|GetActorOfClass "/Game/Blueprints/Raft/BP_Raft_Base1.BP_Raft_Base1_C"))
  (Physics|AddForce (Variables|/Game/Blueprints/Raft/BP_Raft_Base1.BP_Raft_Base1_C|GetSM_Raft _returnvalue) (Math|Vector|RotateVector (Math|Vector|MakeVector (Variables|Default|GetImpulse) 0.0 0.0) (Transformation|GetActorRotation _returnvalue)) "None" true))

(fn RotateRaft
  (bind _returnvalue (Actor|GetActorOfClass "/Game/Blueprints/Raft/BP_Raft_Base1.BP_Raft_Base1_C"))
  (Class|PrimitiveComponent|AddTorqueinDegrees (Variables|/Game/Blueprints/Raft/BP_Raft_Base1.BP_Raft_Base1_C|GetSM_Raft _returnvalue) (Math|Vector|MakeVector 0.0 0.0 (* (Variables|Default|GetImpulse) 2.0)) "None" true))

(fn AleatoireJeux
  (if (Variables|Default|GetModeProtecteur)
    (LocalVariables|SetRandomMinigame (.OutItem (Utilities|Array|Random (Variables|Default|GetMiniJeuProtecteur))))
    (else
      (LocalVariables|SetRandomMinigame (.OutItem (Utilities|Array|Random (Variables|Default|GetMiniJeuSaboteur))))))
  (bind _returnvalue (UserInterface|CreateWidget (LocalVariables|GetRandomMinigame)))
  (UserInterface|Viewport|AddtoViewport _returnvalue 0))