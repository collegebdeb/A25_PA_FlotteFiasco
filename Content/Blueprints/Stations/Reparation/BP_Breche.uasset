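; Raft breach actor that attaches to BP_Raft_Base1, needs a random amount of wood and rope to repair, and periodically drains raft energy until fixed.
; Overlapping players carrying a matching in-use pickup consume it, lowering the count with sound and widget animation.
; A fast looping timer refreshes the WB_Breche display and destroys the breach once both counts reach zero.
; Destruction awards score to the last overlapping player.
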(event Custom|Assemblage
  ;[0.15 0.15 0.15 0.5] Verifie si il y a des ressources qu'il manque pour reparer le bateau
  (if (and (== (Variables|Default|GetNombresBois) 0) (== (Variables|Default|GetNombreCordes) 0))
    (Actor|DestroyActor)))

(event Custom|Malus
  ;[0.15 0.15 0.15 0.5] Apres 5 secondes enleve de l'endurance si la breche n'est pas reparer
  (bind _aswb_energy (Utilities|Casting|CastToWB_Energy (UserInterface|GetWidget (Variables|/Game/Blueprints/Raft/BP_Raft_Base1.BP_Raft_Base1_C|GetWidgetEnergy (Variables|Default|GetBP_Raft)))))
  (Default|RemoveEnergy _aswb_energy 5.0))

(event Custom|UpdateUIValues
  (bind _nombresbois (Variables|Default|GetNombresBois))
  (bind _nombrecordes (Variables|Default|GetNombreCordes))
  ;[0.15 0.15 0.15 0.5] Update le texte de l'UI des breches
  (bind _aswb_breche (Utilities|Casting|CastToWB_Breche (UserInterface|GetWidget (Variables|Default|GetWidget_0))))
  (if (== _nombresbois 0)
    (Widget|SetVisibility (Variables|/Game/Blueprints/Stations/Reparation/WB_Breche.WB_Breche_C|GetImage_Wood _aswb_breche) "Hidden")
    (else
      (Rendering|Components|TextRender|SetText (Variables|/Game/Blueprints/Stations/Reparation/WB_Breche.WB_Breche_C|GetTextWood _aswb_breche) (Utilities|Text|ToText(Integer) _nombresbois))
      (Widget|SetVisibility (Variables|/Game/Blueprints/Stations/Reparation/WB_Breche.WB_Breche_C|GetImage_Wood _aswb_breche) "Visible")))
  (if (== _nombrecordes 0)
    (Widget|SetVisibility (Variables|/Game/Blueprints/Stations/Reparation/WB_Breche.WB_Breche_C|GetImage_Corde _aswb_breche) "Hidden")
    (else
      (Rendering|Components|TextRender|SetText (Variables|/Game/Blueprints/Stations/Reparation/WB_Breche.WB_Breche_C|GetTextCorde _aswb_breche) (Utilities|Text|ToText(Integer) _nombrecordes))
      (Widget|SetVisibility (Variables|/Game/Blueprints/Stations/Reparation/WB_Breche.WB_Breche_C|GetTextCorde _aswb_breche) "Visible"))))

(event Custom|Refresh%20UI
  ;[0.15 0.15 0.15 0.5] Apres 5 secondes enleve de l'endurance si la breche n'est pas reparer
  (CallFunction|Assemblage)
  (CallFunction|UpdateUIValues))

(event EventBeginPlay
  ;[0.15 0.15 0.15 0.5] Apres 5 secondes enleve de l'endurance si la breche n'est pas reparer
  (bind _returnvalue (Actor|GetActorOfClass "/Game/Blueprints/Raft/BP_Raft_Base1.BP_Raft_Base1_C"))
  (Variables|Default|SetBP_Raft _returnvalue)
  (Utilities|Time|SetTimerbyEvent (delegate Custom|Malus) 1e+01 true)
  (CallFunction|UpdateUIValues)
  (Utilities|Time|SetTimerbyEvent (delegate Custom|Refresh%20UI) 0.1 true))

(event EventDestroyed
  ;[0.15 0.15 0.15 0.5] Quand la breche est reparer, joue un son et enleve le nombre de breche en jeu
  (Default|UpdateScore (Variables|Default|GetPlayerRepairing) 1e+01 false)
  (Audio|PlaySound2D "/Game/Sounds/SFX/SFX_RepairAssembling.SFX_RepairAssembling" 0.5 1.0 0.0 0 0))

(event Collision|EventActorBeginOverlap
  (params (OtherActor :type Actor%20Object%20Reference))
  ;[0.15 0.15 0.15 0.5] Quand le joueur a une ressource et qu'il touche une breche, cela commence la reparation de la breche
  (bind _asbp_third_person_character (Utilities|Casting|CastToBP_ThirdPersonCharacter OtherActor))
  (bind _output_get (Variables|Default|SetPlayerRepairing _asbp_third_person_character))
  (bind _bp_pickup (Variables|/Game/ThirdPerson/Blueprints/BP_ThirdPersonCharacter.BP_ThirdPersonCharacter_C|GetBP_PickUp _output_get)
    (:then
      (Variables|Default|SetBP%20Pick%20Up _bp_pickup)
      (Variables|Default|SetPickUpClass (Utilities|GetClass (Variables|Default|GetBP%20Pick%20Up)))
      (if (Variables|/Game/Blueprints/Interactable/Parent/BP_Interactable_PickUp.BP_Interactable_PickUp_C|GetinUse? (Variables|Default|GetBP%20Pick%20Up))
        (Utilities|FlowControl|Sequence
          (:then_0
            ;;[0.15 0.15 0.15 0.5] Si c'est une corde, baisse le nombres de cordes manquantes a la reparation
            (if (and (== (Variables|Default|GetPickUpClass) "/Game/Blueprints/Interactable/BP_PickUp_Rope.BP_PickUp_Rope_C") (> (Variables|Default|GetNombreCordes) 0))
              (bind _result (Math|Integer|DecrementInt (Variables|Default|GetNombreCordes))
                (:%20%20
                  (Variables|Default|SetNombreCordes (Math|Integer|Clamp(Integer) _result 0 5))
                  (Audio|PlaySound2D "/Game/Sounds/SFX/SFX_RopeRepair.SFX_RopeRepair" 0.3 1.0 0.0 0 0)
                  (bind _aswb_breche (Utilities|Casting|CastToWB_Breche (UserInterface|GetWidget (Variables|Default|GetWidget_0))))
                  (UserInterface|Animation|PlayAnimation _aswb_breche (Variables|/Game/Blueprints/Stations/Reparation/WB_Breche.WB_Breche_C|GetRopeDropped _aswb_breche) 0.0 1 "Forward" 1.0 false)
                  (CallFunction|UpdateUIValues :!label _label)
                  (Actor|DestroyActor (Variables|Default|GetBP%20Pick%20Up))
                  (Variables|/Game/ThirdPerson/Blueprints/BP_ThirdPersonCharacter.BP_ThirdPersonCharacter_C|SetisItemHolded? _output_get false)))
              (else
                (CallFunction|UpdateUIValues))))
          (:then_1
            ;;[0.15 0.15 0.15 0.5] Si c'est du bois, baisse le nombres de bois manquants a la reparation
            (if (and (== (Variables|Default|GetPickUpClass) "/Game/Blueprints/Interactable/BP_PickUp_Wood.BP_PickUp_Wood_C") (> (Variables|Default|GetNombresBois) 0))
              (bind _result_2 (Math|Integer|DecrementInt (Variables|Default|GetNombresBois))
                (:%20%20
                  (Variables|Default|SetNombresBois (Math|Integer|Clamp(Integer) _result_2 0 5))
                  (Audio|PlaySound2D "/Game/Sounds/SFX/SFX_WoodRepair.SFX_WoodRepair" 1.0 1.0 0.0 0 0)
                  (bind _aswb_breche_2 (Utilities|Casting|CastToWB_Breche (UserInterface|GetWidget (Variables|Default|GetWidget_0))))
                  (UserInterface|Animation|PlayAnimation _aswb_breche_2 (Variables|/Game/Blueprints/Stations/Reparation/WB_Breche.WB_Breche_C|GetWoodDropped _aswb_breche_2) 0.0 1 "Forward" 1.0 false)
                  (goto _label)))
              (else
                (CallFunction|UpdateUIValues)))))))
    (:else)))

(fn ConstructionScript
  (Variables|Default|SetNombreCordes (Math|Random|RandomIntegerinRange 1 2))
  (Variables|Default|SetNombresBois (Math|Random|RandomIntegerinRange 1 2))
  (bind _returnvalue (Actor|GetActorOfClass "/Game/Blueprints/Raft/BP_Raft_Base1.BP_Raft_Base1_C"))
  (Transformation|AttachActorToActor _returnvalue "None" "KeepWorld" "KeepWorld" "KeepWorld" true))