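; Cooking pickup that runs a two-stage minigame while its overlap zone is active.
; Interacting shows the Animal's DT_Cook inputs as three color-coded planes.
; I/J/K/L build a combo string, cleared after a delay; matching the row's Sequence starts the WB_Cuisine timing bar.
; Tick polls a brief Interact flag against the bar's middle window to reset and hide the minigame, and prints the combo for debugging.
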(event Custom|InputAfficher
  (bind _plane (Variables|Default|GetPlane))
  (bind _plane1 (Variables|Default|GetPlane1))
  (bind _plane2 (Variables|Default|GetPlane2))
  ;[0.15 0.15 0.15 0.5] Update le combo afficher (Feedback de combo)
  (bind _returnvalue (Utilities|GetDataTableRow "/Game/Blueprints/CuisineEtPeche/Outils/Cuisine/DT_Cook.DT_Cook" (Variables|Default|GetAnimal))
    (:then
      (Rendering|SetVisibility (Variables|Default|GetPlane2) true false)
      (Utilities|FlowControl|Sequence
        (:then_0
          (if (Utilities|Enum|Equal(Enum) (.premierinput _returnvalue) "Up")
            (Rendering|Material|SetMaterial _plane 0 "/Game/Blueprints/CuisineEtPeche/Outils/Mat/M_Vert.M_Vert")
            (elif (Utilities|Enum|Equal(Enum) (.premierinput _returnvalue) "Down")
              (Rendering|Material|SetMaterial _plane 0 "/Game/Blueprints/CuisineEtPeche/Outils/Mat/M_Rouge.M_Rouge")
              (elif (Utilities|Enum|Equal(Enum) (.premierinput _returnvalue) "Left")
                (Rendering|Material|SetMaterial _plane 0 "/Game/Blueprints/CuisineEtPeche/Outils/Mat/M_Jaune.M_Jaune")
                (elif (Utilities|Enum|Equal(Enum) (.premierinput _returnvalue) "Right")
                  (Rendering|Material|SetMaterial _plane 0 "/Game/Blueprints/CuisineEtPeche/Outils/Mat/M_Bleu.M_Bleu")
                  (elif (Utilities|Enum|Equal(Enum) (.premierinput _returnvalue) "")
                    (Rendering|SetVisibility (Variables|Default|GetPlane) false false)))))))
        (:then_1
          (if (Utilities|Enum|Equal(Enum) (.deuxiemeinput _returnvalue) "Up")
            (Rendering|Material|SetMaterial _plane1 0 "/Game/Blueprints/CuisineEtPeche/Outils/Mat/M_Vert.M_Vert")
            (elif (Utilities|Enum|Equal(Enum) (.deuxiemeinput _returnvalue) "Down")
              (Rendering|Material|SetMaterial _plane1 0 "/Game/Blueprints/CuisineEtPeche/Outils/Mat/M_Rouge.M_Rouge")
              (elif (Utilities|Enum|Equal(Enum) (.deuxiemeinput _returnvalue) "Left")
                (Rendering|Material|SetMaterial _plane1 0 "/Game/Blueprints/CuisineEtPeche/Outils/Mat/M_Jaune.M_Jaune")
                (elif (Utilities|Enum|Equal(Enum) (.deuxiemeinput _returnvalue) "Right")
                  (Rendering|Material|SetMaterial _plane1 0 "/Game/Blueprints/CuisineEtPeche/Outils/Mat/M_Bleu.M_Bleu")
                  (elif (Utilities|Enum|Equal(Enum) (.deuxiemeinput _returnvalue) "")
                    (Rendering|SetVisibility (Variables|Default|GetPlane1) false false)))))))
        (:then_2
          (if (Utilities|Enum|Equal(Enum) (.troisiemeinput _returnvalue) "Up")
            (Rendering|Material|SetMaterial _plane2 0 "/Game/Blueprints/CuisineEtPeche/Outils/Mat/M_Vert.M_Vert")
            (elif (Utilities|Enum|Equal(Enum) (.troisiemeinput _returnvalue) "Down")
              (Rendering|Material|SetMaterial _plane2 0 "/Game/Blueprints/CuisineEtPeche/Outils/Mat/M_Rouge.M_Rouge")
              (elif (Utilities|Enum|Equal(Enum) (.troisiemeinput _returnvalue) "Left")
                (Rendering|Material|SetMaterial _plane2 0 "/Game/Blueprints/CuisineEtPeche/Outils/Mat/M_Jaune.M_Jaune")
                (elif (Utilities|Enum|Equal(Enum) (.troisiemeinput _returnvalue) "Right")
                  (Rendering|Material|SetMaterial _plane2 0 "/Game/Blueprints/CuisineEtPeche/Outils/Mat/M_Bleu.M_Bleu")
                  (elif (Utilities|Enum|Equal(Enum) (.troisiemeinput _returnvalue) "")
                    (Rendering|SetVisibility (Variables|Default|GetPlane2) false false)))))))))
    (:RowNotFound
      (Rendering|Material|SetMaterial (Variables|Default|GetPlane2) 0 "/Game/LevelPrototyping/Materials/MI_DefaultColorway.MI_DefaultColorway"))))

(event Custom|Assaissonement
  (bind _widget (Variables|Default|GetWidget))
  ;[0.15 0.15 0.15 0.5] Verifie si le combo du joueur est pareil a celui de l'animal dans la data table (Mini jeu part 1)
  (bind _returnvalue (Utilities|GetDataTableRow "/Game/Blueprints/CuisineEtPeche/Outils/Cuisine/DT_Cook.DT_Cook" (Variables|Default|GetAnimal))
    (:then
      (if (and (Utilities|Enum|Equal(Enum) (.sequence _returnvalue) (Variables|Default|GetCombo)) (Variables|Default|GetZone))
        (Rendering|SetVisibility (Variables|Default|GetPlane2) false false)
        (Rendering|SetVisibility _widget true false)
        (bind _aswb_cuisine (Utilities|Casting|CastToWB_Cuisine (UserInterface|GetWidget _widget)))
        (Default|Cook _aswb_cuisine)
        (Variables|Default|SetCombo "")))))

(event Custom|Cuisson
  ;[0.15 0.15 0.15 0.5] Si le joueur appuie sur la touche d'interaction dans le millieu du mini jeu il gagne (Mini jeu part 2)
  (bind _aswb_cuisine (Utilities|Casting|CastToWB_Cuisine (UserInterface|GetWidget (Variables|Default|GetWidget))))
  (if (Math|Boolean|ANDBoolean (> (Variables|/Script/UMG.ProgressBar|GetPercent (Variables|/Game/Blueprints/CuisineEtPeche/Outils/Cuisine/WB_Cuisine.WB_Cuisine_C|GetProgressBar_0 _aswb_cuisine)) 0.45) (< (Variables|/Script/UMG.ProgressBar|GetPercent (Variables|/Game/Blueprints/CuisineEtPeche/Outils/Cuisine/WB_Cuisine.WB_Cuisine_C|GetProgressBar_0 _aswb_cuisine)) 0.55) (Variables|Default|GetInteraction))
    (Default|ResetCuisson _aswb_cuisine)
    (Rendering|SetVisibility (Variables|Default|GetWidget) false false)))

(event Input|EnhancedActionEvents|EnhancedInputActionIA_Interact
  (params (ActionValue :type Boolean) (ElapsedSeconds :type Float%20%28double-precision%29) (TriggeredSeconds :type Float%20%28double-precision%29) (InputAction :type Input%20Action%20Object%20Reference :default "/Game/Input/Actions/IA_Interact.IA_Interact"))
  ;[0.15 0.15 0.15 0.5] Si le joueur appuie sur la touche d'interaction, les input du poisson ss'affiche mais pas si il ya le widget de timing qui est la
  (:Started
    (Utilities|FlowControl|Sequence
      (:then_0
        (Variables|Default|SetInteraction true)
        (Utilities|FlowControl|Delay 0.1)
        (Variables|Default|SetInteraction false))
      (:then_1
        (if (and (Variables|Default|GetZone) (not (Rendering|IsVisible (Variables|Default|GetWidget))))
          (CallFunction|InputAfficher))))))

(event EventBeginPlay
  ;[0.15 0.15 0.15 0.5] Permet de recuperer les input du personnage dans le blueprint ici
  (|CallParentFunction)
  (Input|EnableInput (Game|GetPlayerController 0)))

(event Collision|EventActorBeginOverlap
  (params (OtherActor :type Actor%20Object%20Reference))
  ;[0.15 0.15 0.15 0.5] Si le joueur entre dans la zone le boolean est actif
  (|CallParentFunction OtherActor)
  (Variables|Default|SetZone true))

(event EventTick
  (params (DeltaSeconds :type Float%20%28single-precision%29))
  ;[0.15 0.15 0.15 0.5] Verifie si on peut cuisiner et print des info a l'ecran
  (|CallParentFunction DeltaSeconds)
  (CallFunction|Cuisson)
  (Development|PrintString (Utilities|String|Append "combo :" (Variables|Default|GetCombo)) true true "(R=0.000000,G=0.660000,B=1.000000,A=1.000000)" 0.0))

(event Collision|EventActorEndOverlap
  (params (OtherActor :type Actor%20Object%20Reference))
  ;[0.15 0.15 0.15 0.5] Quand le joueur quitte la zone, les visuels disparaissent
  (Utilities|Casting|CastToBP_ThirdPersonCharacter OtherActor)
  (Rendering|SetVisibility (Variables|Default|GetPlane) false false)
  (Variables|Default|SetZone false)
  (Variables|Default|SetCombo ""))

(event Input|KeyboardEvents|I
  (params (Key :type Key%20Structure :default "None"))
  ;[0.15 0.15 0.15 0.5] Change le combo en fonction des touches utiliser et le reset apres 2 seconde (Update de combo)
  (:Pressed
    (Variables|Default|SetCombo (Utilities|String|Append (Variables|Default|GetCombo) "Up"))
    (CallFunction|Assaissonement)
    (Utilities|FlowControl|Delay 2.0)
    (Variables|Default|SetCombo "")))

(event Input|KeyboardEvents|K
  (params (Key :type Key%20Structure :default "None"))
  ;[0.15 0.15 0.15 0.5] Change le combo en fonction des touches utiliser et le reset apres 2 seconde (Update de combo)
  (:Pressed
    (Variables|Default|SetCombo (Utilities|String|Append (Variables|Default|GetCombo) "Down"))
    (CallFunction|Assaissonement)
    (Utilities|FlowControl|Delay 2.0)
    (Variables|Default|SetCombo "")))

(event Input|KeyboardEvents|J
  (params (Key :type Key%20Structure :default "None"))
  ;[0.15 0.15 0.15 0.5] Change le combo en fonction des touches utiliser et le reset apres 2 seconde (Update de combo)
  (:Pressed
    (Variables|Default|SetCombo (Utilities|String|Append (Variables|Default|GetCombo) "Left"))
    (CallFunction|Assaissonement)
    (Utilities|FlowControl|Delay 2.0)
    (Variables|Default|SetCombo "")))

(event Input|KeyboardEvents|L
  (params (Key :type Key%20Structure :default "None"))
  ;[0.15 0.15 0.15 0.5] Change le combo en fonction des touches utiliser et le reset apres 2 seconde (Update de combo)
  (:Pressed
    (Variables|Default|SetCombo (Utilities|String|Append (Variables|Default|GetCombo) "Right"))
    (CallFunction|Assaissonement)
    (Utilities|FlowControl|Delay 2.0)
    (Variables|Default|SetCombo "")))

(fn ConstructionScript
  (|CallParentFunction))