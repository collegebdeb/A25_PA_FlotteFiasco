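; BP_BrecheSpawns is a raft spawner actor that places BP_Breche breach actors at random points inside its Box component.
; On BeginPlay it calls the SpawnB event with ActorsToSpawn as the loop count.
; Each iteration spawns a fixed-rotation breach, adjusted for collisions but always spawned, and increments BrechesInGame, skipping when that counter equals five.
; Nothing in this graph decrements the counter.
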(event Custom|SpawnB
  (params (NombreDeLoop :type Integer))
  (bind _box (Variables|Default|GetBox))
  (for _index (range 1 NombreDeLoop)
    (if (not (== (Variables|Default|GetBrechesInGame) 5))
      (Game|SpawnActorfromClass "/Game/Blueprints/Raft/BP_Breche.BP_Breche_C" (Math|Transform|MakeTransform (Math|Random|RandomPointinBoundingBox (Transformation|GetWorldLocation _box) (Variables|/Script/Engine.BoxComponent|GetBoxExtent _box)) "0.000000,-90.000000,0.000000" "1.000000,1.000000,1.000000") "AdjustIfPossibleButAlwaysSpawn" "MultiplyWithRoot" 0 0)
      (bind _result (Math|Integer|IncrementInt (Variables|Default|GetBrechesInGame))
        (:%20%20
          (Variables|Default|SetBrechesInGame _result))))))

(event Collision|EventActorBeginOverlap
  (params (OtherActor :type Actor%20Object%20Reference)))

(event EventTick
  (params (DeltaSeconds :type Float%20%28single-precision%29)))

(event EventBeginPlay
  (CallFunction|SpawnB (Variables|Default|GetActors%20to%20Spawn)))

(fn ConstructionScript)