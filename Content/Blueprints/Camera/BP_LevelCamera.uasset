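; Level camera that takes over the player view and follows the raft down the river, or sits at a fixed position without one.
; Tick interpolates toward the raft plus an offset, freezing when too far and holding Z near the set height to absorb buoyancy bobbing.
; UpdateCamTransform, meant for trigger boxes, starts a timer blending offset and rotation by the camera's distance-based progress between two points, until ClearCamUpdate stops it.
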(event Custom|UpdateCamTransform
  (params (InitialTransform :type Transform) (FinalTransform :type Transform) (PointDepart :type Vector) (PointFinal :type Vector))
  ;[0.15 0.15 0.15 0.5] Update le transform de la caméra de façon smooth selon la direction de la rivière - a call sur des trigger box une pour départ une pour final
  (Utilities|FlowControl|Sequence
    (:then_0
      (Variables|Default|SetInitial%20Transform InitialTransform)
      (Variables|Default|SetFinal%20Transform FinalTransform)
      (Variables|Default|SetPoint%20Depart PointDepart)
      (Variables|Default|SetPoint%20Final PointFinal))
    (:then_1
      (bind _returnvalue (Utilities|Time|SetTimerbyEvent (delegate Custom|LerpCam) 0.01 true))
      (Variables|Default|SetTimer _returnvalue))))

(event Custom|LerpCam
  (bind _returnvalue (Transformation|GetActorLocation))
  (bind _initial_transform (Variables|Default|GetInitial%20Transform))
  (bind _final_transform (Variables|Default|GetFinal%20Transform))
  (bind _point_final (Variables|Default|GetPoint%20Final))
  (bind _point_depart (Variables|Default|GetPoint%20Depart))
  (bind _point_final_2 (Variables|Default|GetPoint%20Final))
  (bind _returnvalue_2 (Math|Vector|Distance(Vector) _point_depart _point_final_2))
  (bind _returnvalue_3 (Math|Vector|Distance(Vector) _returnvalue _point_final))
  (bind _returnvalue_4 (/ _returnvalue_3 _returnvalue_2))
  (bind _returnvalue_5 (- 1.0 _returnvalue_4))
  (bind _returnvalue_6 (Math|Transform|Lerp(Transform) _initial_transform _final_transform _returnvalue_5))
  ;[0.15 0.15 0.15 0.5] Update le transform de la caméra de façon smooth selon la direction de la rivière - a call sur des trigger box une pour départ une pour final
  (Variables|Default|SetCameraPosFromRaft (.location _returnvalue_6))
  (Transformation|SetActorRotation (.rotation _returnvalue_6)))

(event Custom|ClearCamUpdate
  (bind _timer (Variables|Default|GetTimer))
  ;[0.15 0.15 0.15 0.5] Réinitialise le timer
  (if (Utilities|Time|IsValidTimerHandle _timer)
    (Utilities|Time|ClearandInvalidateTimerbyHandle _timer)))

(event EventBeginPlay
  ;[0.15 0.15 0.15 0.5] Recupere le radeau pour le suivre ensuite, s'il n'y a pas de radeau dans la scene place la camera dans une position qu'on souhaite
  (Game|Player|SetViewTargetwithBlend (Game|GetPlayerController 0) self 0.0 "VTBlend_Linear" 0.0 false)
  (bind _returnvalue (Actor|GetActorOfClass "/Game/Blueprints/Raft/BP_Raft_Base1.BP_Raft_Base1_C"))
  (bind _output_get (Variables|Properties|SetTargetActor _returnvalue))
  (Utilities|IsValid _output_get
    (:Is%20Valid
      (Transformation|SetActorLocation (Math|Vector|MakeVector (.x (Transformation|GetActorLocation _output_get)) (.y (Transformation|GetActorLocation _output_get)) (+ (.z (Transformation|GetActorLocation _output_get)) (Variables|Properties|GetHauteurCameraFromRaft))) false false)
      (Variables|Default|SetTransformAtCheckPoint (Transformation|GetActorTransform)))
    (:Is%20Not%20Valid
      (Transformation|SetActorLocation (Math|Vector|MakeVector 795.0 17.0 1583.0) false false)
      (Variables|Default|SetTransformAtCheckPoint (Transformation|GetActorTransform)))))

(event EventTick
  (params (DeltaSeconds :type Float%20%28single-precision%29))
  (bind _self self)
  (bind _self_2 self)
  (bind _cameraposfromraft (Variables|Default|GetCameraPosFromRaft))
  (bind _targetactor (Variables|Properties|GetTargetActor))
  (bind _targetactor_2 (Variables|Properties|GetTargetActor))
  (bind _returnvalue (Transformation|GetActorLocation _targetactor))
  (bind _returnvalue_2 (Transformation|GetActorLocation _self))
  (bind _returnvalue_3 (Transformation|GetActorLocation _targetactor_2))
  (bind _returnvalue_4 (Transformation|GetActorLocation _self_2))
  (bind _returnvalue_5 (Math|Vector|Distance(Vector) _returnvalue_3 _returnvalue_2))
  (bind _returnvalue_6 (+ _returnvalue _cameraposfromraft))
  (bind _returnvalue_7 (>= _returnvalue_5 5e+03))
  (bind _returnvalue_8 (Math|Float|SelectFloat 0.0 5.0 _returnvalue_7))
  (bind _returnvalue_9 (Math|Interpolation|VInterpTo _returnvalue_4 _returnvalue_6 DeltaSeconds _returnvalue_8))
  ;[0.15 0.15 0.15 0.5] Fait suivre la camera avec le radeau
  (Variables|Properties|GetTargetActor
    (:then
      (Transformation|SetActorLocation (Math|Vector|MakeVector (.x _returnvalue_9) (.y _returnvalue_9) (Math|Float|SelectFloat (.Z (Math|Vector|BreakVector (Transformation|GetActorLocation self))) (.z _returnvalue_9) (Math|Float|NearlyEqual(Float) (Math|Float|Absolute(Float) (.z (- (Transformation|GetActorLocation (Variables|Properties|GetTargetActor)) (Transformation|GetActorLocation self)))) (Variables|Properties|GetHauteurCameraFromRaft) 1e+02))) false false))
    (:else)))

(fn ConstructionScript)