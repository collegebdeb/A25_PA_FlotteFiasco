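; Spawner that periodically places actors of a configurable class, likely rafts given the asset name, at random points inside its Box component.
; BeginPlay starts a looping timer with a random interval between TempsMin and TempsMax, rolled only once.
; Each tick of that timer attempts one or two spawns with a fixed rotation, adjusting for collisions.
; NumberOfActors only increments, so MaxActors caps total lifetime spawns.
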(event Custom|SpawnB
  (bind _box (Variables|Default|GetBox))
  (for _index (range 0 (Math|Random|RandomIntegerinRange 0 1))
    (if (not (== (Variables|Default|GetNumberOfActors) (Variables|Default|GetMaxActors)))
      (Game|SpawnActorfromClass (Variables|Default|GetActorToSpawn) (Math|Transform|MakeTransform (Math|Random|RandomPointinBoundingBox (Transformation|GetWorldLocation _box) (Variables|/Script/Engine.BoxComponent|GetBoxExtent _box)) "0.000000,-180.000000,0.000000" "1.000000,1.000000,1.000000") "AdjustIfPossibleButAlwaysSpawn" "MultiplyWithRoot" 0 0)
      (bind _result (Math|Integer|IncrementInt (Variables|Default|GetNumberOfActors))
        (:%20%20
          (Variables|Default|SetNumberOfActors _result))))))

(event Collision|EventActorBeginOverlap
  (params (OtherActor :type Actor%20Object%20Reference)))

(event EventTick
  (params (DeltaSeconds :type Float%20%28single-precision%29)))

(event EventBeginPlay
  (Utilities|Time|SetTimerbyEvent (delegate Custom|SpawnB) (Math|Conversions|ToFloat(Integer) (Math|Random|RandomIntegerinRange (Variables|Default|GetTempsMin) (Variables|Default|GetTempsMax))) true))

(fn ConstructionScript)