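; BP_PickUp_Poisson is a fish pickup that players can pick up and drop.
; It is a child Blueprint that passes overlap, PickUp and Drop events to its parent's logic.
; After the parent call, PickUp sets the player's HasFish flag to true and Drop sets it to false.
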(event EventBeginPlay)

(event Collision|EventActorBeginOverlap
  (params (OtherActor :type Actor%20Object%20Reference))
  (|CallParentFunction OtherActor))

(event EventTick
  (params (DeltaSeconds :type Float%20%28single-precision%29))
  (|CallParentFunction DeltaSeconds) ; This node is disabled and will not be called.\nDrag off pins to build functionality.
)

(event EventDrop
  (params (Player :type BP%20Third%20Person%20Character%20Object%20Reference))
  (|CallParentFunction Player)
  (Variables|/Game/ThirdPerson/Blueprints/BP_ThirdPersonCharacter.BP_ThirdPersonCharacter_C|SethasFish? Player false))

(event EventPickUp
  (params (Player :type BP%20Third%20Person%20Character%20Object%20Reference))
  (|CallParentFunction Player)
  (Variables|/Game/ThirdPerson/Blueprints/BP_ThirdPersonCharacter.BP_ThirdPersonCharacter_C|SethasFish? Player true))

(event EventActorEndOverlap
  (params (OtherActor :type Actor%20Object%20Reference))
  (|CallParentFunction OtherActor))

(fn ConstructionScript
  (|CallParentFunction))