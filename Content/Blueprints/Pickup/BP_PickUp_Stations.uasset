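; BP_PickUp_Stations is a pickup child Blueprint for stations that lock the player in place when picked up.
; PickUp disables the player's character movement and sets its DisabledMovement flag, while Drop only prints a debug string and does not restore movement.
; Box overlaps are forwarded to the parent's overlap handling.
; The construction script runs the parent's setup, then turns off physics simulation on the SM mesh.
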(event OnComponentBeginOverlap(Box)
  (params (OverlappedComponent :type Primitive%20Component%20Object%20Reference) (OtherActor :type Actor%20Object%20Reference) (OtherComp :type Primitive%20Component%20Object%20Reference) (OtherBodyIndex :type Integer) (bFromSweep :type Boolean) (SweepResult :type Hit%20Result%20Structure%20%28by%20ref%29))
  (|CallParentFunction OtherActor))

(event EventBeginPlay)

(event Collision|EventActorBeginOverlap
  (params (OtherActor :type Actor%20Object%20Reference)))

(event EventPickUp
  (params (Player :type BP%20Third%20Person%20Character%20Object%20Reference))
  (Pawn|Components|CharacterMovement|DisableMovement (Variables|/Script/Engine.Character|GetCharacterMovement (Variables|Default|GetPlayer)))
  (Variables|/Game/ThirdPerson/Blueprints/BP_ThirdPersonCharacter.BP_ThirdPersonCharacter_C|SetdisabledMovement? (Variables|Default|GetPlayer) true))

(event EventDrop
  (params (Player :type BP%20Third%20Person%20Character%20Object%20Reference))
  (Development|PrintString "drop in bp_station" true true "(R=0.000000,G=0.660000,B=1.000000,A=1.000000)" 0.0))

(fn ConstructionScript
  (|CallParentFunction)
  (Physics|SetSimulatePhysics (Variables|Default|GetSM) false))