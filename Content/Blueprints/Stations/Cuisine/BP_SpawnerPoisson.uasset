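; BP_SpawnerPoisson is a fishing spot that turns into a fish pickup when the fishing mini-game completes.
; Its Spawn event checks the WB_Peche widget's progress bar and, once full, destroys the actor and stops ignoring the player's move input.
; The Destroyed event spawns BP_PickUp_Poisson above the cube and launches it upward, so any destruction yields a fish.
; SeeFeedback toggles the widget's visibility.
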(event Custom|Spawn
  ;[0.15 0.15 0.15 0.5] Quand la progression du mini jeu est complete, cela detruit l'acteur ce qui declenche l'event destroyed
  (bind _aswb_peche (Utilities|Casting|CastToWB_Peche (UserInterface|GetWidget (Variables|Default|GetWidget))))
  (if (>= (Variables|/Script/UMG.ProgressBar|GetPercent (Variables|/Game/Blueprints/Stations/Peche/WB_Peche.WB_Peche_C|GetProgressBar_37 _aswb_peche)) 1.0)
    (Actor|DestroyActor)
    (Input|SetIgnoreMoveInput (Game|GetPlayerController 0) false)))

(event Custom|SeeFeedback
  (params (bNewVisibility :type Boolean))
  (Rendering|SetVisibility (Variables|Default|GetWidget) bNewVisibility false))

(event EventBeginPlay)

(event Collision|EventActorBeginOverlap
  (params (OtherActor :type Actor%20Object%20Reference)))

(event EventTick
  (params (DeltaSeconds :type Float%20%28single-precision%29)))

(event EventDestroyed
  ;[0.15 0.15 0.15 0.5] Quand l'actor est détruit cela fait spawn un vrai poisson
  (bind _returnvalue (Game|SpawnActorfromClass "/Game/Blueprints/Interactable/BP_PickUp_Poisson.BP_PickUp_Poisson_C" (Math|Conversions|ToTransform(Vector) (+ (Transformation|GetWorldLocation (Variables|Default|GetCube)) "0.000000,0.000000,100.000000")) "Undefined" "MultiplyWithRoot" 0 0))
  (Physics|AddForce (Variables|/Game/Blueprints/Interactable/Parent/BP_Interactable_PickUp.BP_Interactable_PickUp_C|GetSM _returnvalue) "0.000000,0.000000,15000000.000000" "None" false))

(fn ConstructionScript)