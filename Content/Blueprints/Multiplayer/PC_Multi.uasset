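; Player controller for local multiplayer that lets each player drop into the game on the join input.
; Joining, if not dead and without a pawn, spawns the player at the raft's respawn point, applies a per-player material, increments GM_Multi's count and adds game, victory and game-over UI entries.
; BeginPlay adds the default Enhanced Input mapping after a short delay.
; The Vagues input fires mobile press and release dispatchers.
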(event Input|EnhancedActionEvents|EnhancedInputActionIA_JoinGame
  (params (ActionValue :type Boolean) (ElapsedSeconds :type Float%20%28double-precision%29) (TriggeredSeconds :type Float%20%28double-precision%29) (InputAction :type Input%20Action%20Object%20Reference :default "/Game/Input/Actions/Multi/IA_JoinGame.IA_JoinGame"))
  (bind _self self)
  (bind _returnvalue (Class|GameplayStatics|GetPlayerControllerID _self))
  (:Started
    (if (not (Variables|Default|GetisDead?))
      (Utilities|IsValid (Pawn|GetControlledPawn)
        (:Is%20Not%20Valid
          (bind _returnvalue_2 (Actor|GetActorOfClass "/Game/Blueprints/Raft/BP_Raft_Base1.BP_Raft_Base1_C"))
          (Class|GameModeBase|RestartPlayeratTransform (Game|GetGameMode) self (Transformation|GetWorldTransform (Variables|/Game/Blueprints/Raft/BP_Raft_Base1.BP_Raft_Base1_C|GetRespawnPoint _returnvalue_2)))
          (Rendering|Material|SetMaterial (Variables|/Script/Engine.Character|GetMesh (Game|GetPlayerCharacter _returnvalue)) 1 (Utilities|Array|Get(acopy) (Variables|Default|GetPlayerColor) _returnvalue))
          (bind _asgm_multi (Utilities|Casting|CastToGM_Multi (Game|GetGameMode)))
          (Math|Integer|IncrementInt (Variables|/Game/Blueprints/Multiplayer/GM_Multi.GM_Multi_C|GetPlayerCount _asgm_multi)
            (:%20%20
              (bind _wb_joingame (Variables|/Game/Blueprints/Multiplayer/GM_Multi.GM_Multi_C|GetWB_JoinGame _asgm_multi)
                (:then
                  (Default|DestroyJoinGameWidget _wb_joingame))
                (:else
                  _))
              (Default|AddPlayersUI (Variables|/Game/Blueprints/Multiplayer/GM_Multi.GM_Multi_C|GetWB_GameUI (Variables|Default|GetGM_Multi)) (Variables|Default|GetLocalPlayerControllerID))
              (Default|AddPlayerVictory (Variables|/Game/Blueprints/Multiplayer/GM_Multi.GM_Multi_C|GetWB_Victory (Variables|Default|GetGM_Multi)) (Variables|Default|GetLocalPlayerControllerID))
              (Default|AddPlayerGameOver (Variables|/Game/Blueprints/Multiplayer/GM_Multi.GM_Multi_C|GetWB_GameOver (Variables|Default|GetGM_Multi)) (Variables|Default|GetLocalPlayerControllerID))
              (Audio|PlaySound2D "/Game/Sounds/SFX/SFX_CartoonYoink.SFX_CartoonYoink" 1.0 1.0 0.0 0 0))))))))

(event EventBeginPlay
  (bind _self self)
  (bind _returnvalue (PlayerController|LocalPlayerSubsystems|GetEnhancedInputLocalPlayerSubsystem _self))
  (Utilities|FlowControl|Delay 0.2)
  (Utilities|IsValid _returnvalue
    (:Is%20Valid
      (Input|AddMappingContext _returnvalue "/Game/Input/IMC_Default.IMC_Default" 0 "(bIgnoreAllPressedKeysUntilRelease=True,bForceImmediately=False,bNotifyUserSettings=False)"))))

(event Input|EnhancedActionEvents|EnhancedInputActionIA_Vagues
  (params (ActionValue :type Vector%202D%20Structure) (ElapsedSeconds :type Float%20%28double-precision%29) (TriggeredSeconds :type Float%20%28double-precision%29) (InputAction :type Input%20Action%20Object%20Reference :default "/Game/Input/Actions/Mobile/IA_Vagues.IA_Vagues"))
  ;[0.15 0.15 0.15 0.5] Vagues
  (:Triggered
    (Default|CallDISPMobilePress :!label _label))
  (:Started
    (goto _label))
  (:Canceled
    (Default|CallDISPMobileRelease :!label _label_2))
  (:Completed
    (goto _label_2)))

(fn ConstructionScript)