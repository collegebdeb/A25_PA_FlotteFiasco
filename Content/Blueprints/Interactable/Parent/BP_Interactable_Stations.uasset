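; Parent Blueprint for interactable stations that a player mans, such that the player is locked in place while using one.
; BeginPlay reads the attach socket, input mapping context and energy impact from DT_Pickup, keyed by station type.
; PickUp, allowed when not in use, attaches the player to the socket, disables movement and adds the station's mapping context; Drop reverses this.
; Overlap events defer to the parent class, and construction turns off mesh physics.
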(event OnComponentBeginOverlap(SphereOverlap)
  (params (OverlappedComponent :type Primitive%20Component%20Object%20Reference) (OtherActor :type Actor%20Object%20Reference) (OtherComp :type Primitive%20Component%20Object%20Reference) (OtherBodyIndex :type Integer) (bFromSweep :type Boolean) (SweepResult :type Hit%20Result%20Structure%20%28by%20ref%29))
  ;[0.15 0.15 0.15 0.5] Begin Overlap - Parent
  (|CallParentFunction OtherActor))

(event OnComponentEndOverlap(SphereOverlap)
  (params (OverlappedComponent :type Primitive%20Component%20Object%20Reference) (OtherActor :type Actor%20Object%20Reference) (OtherComp :type Primitive%20Component%20Object%20Reference) (OtherBodyIndex :type Integer))
  ;[0.15 0.15 0.15 0.5] End Overlap - Parent
  (|CallParentFunction OtherActor))

(event EventBeginPlay
  ;[0.15 0.15 0.15 0.5] Begin Play - Récupère certaines valeurs de la DataTable pour les assigner aux stations.
  (bind _returnvalue (Utilities|GetDataTableRow "/Game/Blueprints/Interactable/Parent/DT_Pickup.DT_Pickup" (Utilities|String|StringToName (Utilities|String|EnumtoString (Variables|Default|GetStation_Type))))
    (:then
      (Variables|Default|SetAttachToSocketName (.SocketName (Utilities|Struct|BreakS_Pickup _returnvalue)))
      (Variables|Default|SetMappingContext (.MappingContext (Utilities|Struct|BreakS_Pickup _returnvalue)))
      (Variables|Default|SetEnergyImpact (.EnergyImpact (Utilities|Struct|BreakS_Pickup _returnvalue))))))

(event EventPickUp
  (params (Player :type BP%20Third%20Person%20Character%20Object%20Reference))
  ;[0.15 0.15 0.15 0.5] Pick Up - Attache le joueur à la station, désactive ses mouvements et assigne l'IMC correspondant à la station.
  (if (not (Variables|Default|GetinUse?))
    (bind _output_get (Variables|Default|SetPlayer Player))
    (Transformation|AttachActorToActor _output_get self (Variables|Default|GetAttachToSocketName) "SnapToTarget" "KeepWorld" "KeepWorld" false)
    (Variables|Default|SetinUse? true)
    (Pawn|Components|CharacterMovement|DisableMovement (Variables|/Script/Engine.Character|GetCharacterMovement (Variables|Default|GetPlayer)))
    (CallFunction|AddMappingContext (Variables|Default|GetPlayer))
    (Default|SetPickupType (Variables|Default|GetPlayer) (Variables|Default|GetPickup_type) self)
    (Variables|/Game/ThirdPerson/Blueprints/BP_ThirdPersonCharacter.BP_ThirdPersonCharacter_C|SetdisabledMovement? (Variables|Default|GetPlayer) true)
    (Audio|PlaySound2D "/Game/Sounds/SFX/ButtonUI.ButtonUI" 1.0 1.0 0.0 0 0)
    (CallFunction|DisableOverlapFeedback)
    (Variables|Default|SetCurrentPlayerIndex (Class|GameplayStatics|GetPlayerControllerID (.AsPC%20Multi (Utilities|Casting|CastToPC_Multi (Pawn|GetController (Variables|Default|GetPlayer))))))))

(event EventDrop
  (params (Player :type BP%20Third%20Person%20Character%20Object%20Reference))
  ;[0.15 0.15 0.15 0.5] Drop - Détache le joueur de la station, rétablit ses mouvements et retire l'IMC de la station.
  (if (Variables|Default|GetinUse?)
    (Transformation|DetachFromActor Player "KeepWorld" "KeepWorld" "KeepWorld")
    (Variables|Default|SetinUse? false)
    (Pawn|Components|CharacterMovement|SetMovementMode (Variables|/Script/Engine.Character|GetCharacterMovement (Variables|Default|GetPlayer)) "MOVE_Walking" 0)
    (CallFunction|RemoveMappingContext (Variables|Default|GetPlayer))
    (Variables|/Game/ThirdPerson/Blueprints/BP_ThirdPersonCharacter.BP_ThirdPersonCharacter_C|SetdisabledMovement? (Variables|Default|GetPlayer) false)
    (Variables|Default|SetPlayer 0)))

(fn ConstructionScript
  (|CallParentFunction)
  (Physics|SetSimulatePhysics (Variables|Default|GetSM) false))