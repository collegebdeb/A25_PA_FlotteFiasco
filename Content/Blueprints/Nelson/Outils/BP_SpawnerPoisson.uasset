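; Fishing spot actor that produces a BP_Cuisine item once the fishing progress bar is full.
; Each tick it reads the progress bar of the WB_Peche UI in its widget component.
; At full, it spawns the item offset from its cube, launches it upward with a physics force, destroys itself and releases the player's move-input lock.
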(event EventBeginPlay)

(event Collision|EventActorBeginOverlap
  (params (OtherActor :type Actor%20Object%20Reference)))

(event EventTick
  (params (DeltaSeconds :type Float%20%28single-precision%29))
  (bind _aswb_peche (Utilities|Casting|CastToWB_Peche (UserInterface|GetWidget (Variables|Default|GetWidget))))
  (if (>= (Variables|/Script/UMG.ProgressBar|GetPercent (Variables|/Game/Outils/WB_Peche.WB_Peche_C|GetProgressBar_37 _aswb_peche)) 1.0)
    (Utilities|FlowControl|DoOnce false
      (:Completed
        (bind _returnvalue (Game|SpawnActorfromClass "/Game/Outils/BP_Cuisine.BP_Cuisine_C" (Math|Conversions|ToTransform(Vector) (+ (Transformation|GetWorldLocation (Variables|Default|GetCube)) "150.000000,0.000000,100.000000")) "Undefined" "MultiplyWithRoot" 0 0))
        (Physics|AddForce (Variables|/Game/Outils/BP_Cuisine.BP_Cuisine_C|GetSphere _returnvalue) "0.000000,0.000000,15000000.000000" "None" false)
        (Actor|DestroyActor)
        (Input|SetIgnoreMoveInput (Game|GetPlayerController 0) false)))))

(fn ConstructionScript)