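; Fishing rod pickup that enables its input on overlap and lets the player cast at fish or fish spawners.
; Holding Interact runs a looping timer that charges cast length on an arrow widget; releasing fires a line trace.
; A hit locks movement: hooked fish are pulled back by physics force on Interact, while spawners gain catch progress through TakeOutFish input.
; Drop or ComboRight releases the line and restores movement.
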(event Custom|Lancer
  (bind _arrow (Variables|Default|GetArrow))
  (bind _returnvalue (Transformation|GetWorldLocation _arrow))
  ;[0.15 0.15 0.15 0.5] Si le lancer est effectuer et touche un objet, il va réagir
  (if (not (Variables|Default|GetAccrocher))
    (bind _outhit (Collision|LineTraceByChannel _returnvalue (+ _returnvalue (* (Math|Vector|GetForwardVector _arrow) (Variables|Default|GetLongueur))) "TraceTypeQuery1" false 0 "Persistent"))
    (Utilities|FlowControl|Sequence
      (:then_0
        ;;[0.15 0.15 0.15 0.5] Si le poisson est toucher on peut le ramener vers nous
        (Utilities|Casting|CastToBP_PickUp_Poisson (.HitActor (Collision|BreakHitResult _outhit)))
        (Input|SetIgnoreMoveInput (Game|GetPlayerController 0) true)
        (Variables|Default|SetAccrocher true))
      (:then_1
        ;;[0.15 0.15 0.15 0.5] Si la zone de poisson est toucher on peut commencer a sortir le poisson de l'eau
        (bind _asbp_spawner_poisson (Utilities|Casting|CastToBP_SpawnerPoisson (.HitActor (Collision|BreakHitResult _outhit))))
        (Default|SeeFeedback _asbp_spawner_poisson true)
        (Input|SetIgnoreMoveInput (Game|GetPlayerController 0) true)
        (Variables|Default|SetPecheEnCours true)))))

(event Custom|FeedbackVisuel
  (bind _widget (Variables|Default|GetWidget))
  ;[0.15 0.15 0.15 0.5] Montre la distance de lancer
  (Rendering|SetVisibility _widget true false)
  (bind _aswb_fleche (Utilities|Casting|CastToWB_Fleche (UserInterface|GetWidget _widget)))
  (Progress|SetPercent (Variables|/Game/Blueprints/CuisineEtPeche/Outils/WB_Fleche.WB_Fleche_C|GetProgressBar_32 _aswb_fleche) (/ (Variables|Default|GetLongueur) 1e+03)))

(event Custom|StatutCorde
  ;[0.15 0.15 0.15 0.5] Quand le joueur appuie sur F cela augmente la distance de lancer
  (if (> (Variables|Default|GetLongueur) 9e+02)
    (Variables|Default|SetLongueur 0.0)
    (else
      (Variables|Default|SetLongueur (+ (Variables|Default|GetLongueur) 1e+02))
      (CallFunction|FeedbackVisuel))))

(event Input|EnhancedActionEvents|EnhancedInputActionIA_Interact
  (params (ActionValue :type Boolean) (ElapsedSeconds :type Float%20%28double-precision%29) (TriggeredSeconds :type Float%20%28double-precision%29) (InputAction :type Input%20Action%20Object%20Reference :default "/Game/Input/Actions/IA_Interact.IA_Interact"))
  (bind _actif (Variables|Default|GetActif))
  ;[0.15 0.15 0.15 0.5] Quand le joueur appuie sur F cela augmente la distance de lancer
  (:Started
    (if (not (Variables|Default|GetAccrocher))
      (if _actif
        (bind _returnvalue (Utilities|Time|SetTimerbyEvent (delegate Custom|StatutCorde) 0.1 true))
        (Variables|Default|SetLongueur 0.0)
        (Rendering|SetVisibility (Variables|Default|GetWidget) true false))))
  (:Completed
    (if _actif
      (Utilities|Time|ClearandInvalidateTimerbyHandle _returnvalue)
      (CallFunction|Lancer)
      (Rendering|SetVisibility (Variables|Default|GetWidget) false false))))

(event Input|EnhancedActionEvents|EnhancedInputActionIA_ComboRight
  (params (ActionValue :type Boolean) (ElapsedSeconds :type Float%20%28double-precision%29) (TriggeredSeconds :type Float%20%28double-precision%29) (InputAction :type Input%20Action%20Object%20Reference :default "/Game/Input/Actions/IA_ComboRight.IA_ComboRight"))
  ;[0.15 0.15 0.15 0.5] Quand le joueur drop l'item ou decroche sa canne a peche, il peut se deplacer
  (:Started
    (Input|SetIgnoreMoveInput (Game|GetPlayerController 0) false)
    (Variables|Default|SetAccrocher false)
    (Variables|Default|SetPecheEnCours false)
    (Default|SeeFeedback (stale Custom|Lancer _asbp_spawner_poisson) false)))

(event Input|EnhancedActionEvents|EnhancedInputActionIA_TakeOutFish
  (params (ActionValue :type Boolean) (ElapsedSeconds :type Float%20%28double-precision%29) (TriggeredSeconds :type Float%20%28double-precision%29) (InputAction :type Input%20Action%20Object%20Reference :default "/Game/Input/Actions/IA_TakeOutFish.IA_TakeOutFish"))
  ;[0.15 0.15 0.15 0.5] Sors le poisson de l'eau
  (bind _asbp_third_person_character (Utilities|Casting|CastToBP_ThirdPersonCharacter (Game|GetPlayerCharacter 0)))
  (if (Math|Boolean|ANDBoolean (Variables|Default|GetPecheEnCours) (> (.z (Math|Vector|GetForwardVector (Math|Rotator|MakeRotator 0.0 0.0 (.yaw (Pawn|GetControlRotation _asbp_third_person_character :!class /Script/Engine.Pawn))))) -2.0) (< (.z (Math|Vector|GetForwardVector (Math|Rotator|MakeRotator 0.0 0.0 (.yaw (Pawn|GetControlRotation _asbp_third_person_character :!class /Script/Engine.Pawn))))) 2.0))
    (bind _asbp_spawner_poisson (Utilities|Casting|CastToBP_SpawnerPoisson (.HitActor (Collision|BreakHitResult (stale Custom|Lancer _outhit)))))
    (bind _aswb_peche (Utilities|Casting|CastToWB_Peche (UserInterface|GetWidget (Variables|/Game/Blueprints/CuisineEtPeche/Outils/Cuisine/BP_SpawnerPoisson.BP_SpawnerPoisson_C|GetWidget _asbp_spawner_poisson))))
    (Variables|/Game/Blueprints/CuisineEtPeche/Outils/WB_Peche.WB_Peche_C|SetProgressionPeche _aswb_peche (+ (Variables|/Game/Blueprints/CuisineEtPeche/Outils/WB_Peche.WB_Peche_C|GetProgressionPeche _aswb_peche) 5.0))
    (Default|Spawn _asbp_spawner_poisson)))

(event Input|EnhancedActionEvents|EnhancedInputActionIA_Drop
  (params (ActionValue :type Boolean) (ElapsedSeconds :type Float%20%28double-precision%29) (TriggeredSeconds :type Float%20%28double-precision%29) (InputAction :type Input%20Action%20Object%20Reference :default "/Game/Input/Actions/IA_Drop.IA_Drop"))
  ;[0.15 0.15 0.15 0.5] Quand le joueur drop l'item ou decroche sa canne a peche, il peut se deplacer
  (:Started
    (Input|SetIgnoreMoveInput (Game|GetPlayerController 0) false)
    (Variables|Default|SetAccrocher false)
    (Variables|Default|SetPecheEnCours false)
    (Default|SeeFeedback (stale Custom|Lancer _asbp_spawner_poisson) false)))

(event Input|EnhancedActionEvents|EnhancedInputActionIA_Interact
  (params (ActionValue :type Boolean) (ElapsedSeconds :type Float%20%28double-precision%29) (TriggeredSeconds :type Float%20%28double-precision%29) (InputAction :type Input%20Action%20Object%20Reference :default "/Game/Input/Actions/IA_Interact.IA_Interact"))
  ;[0.15 0.15 0.15 0.5] Ramene le poisson vers nous
  (:Started
    (if (Variables|Default|GetAccrocher)
      (bind _asbp_pick_up_poisson (Utilities|Casting|CastToBP_PickUp_Poisson (.HitActor (Collision|BreakHitResult (stale Custom|Lancer _outhit)))))
      (Physics|AddForce (Variables|/Game/Blueprints/Pickup/BP_PickUp.BP_PickUp_C|GetSM _asbp_pick_up_poisson) (* (Math|Vector|GetForwardVector (Variables|Default|GetArrow)) -1e+06) "None" false))))

(event Collision|EventActorBeginOverlap
  (params (OtherActor :type Actor%20Object%20Reference))
  ;[0.15 0.15 0.15 0.5] Quand le joueur ramasse l'objet il peut utiliser les fonctions de l'objet en recuperant ses inputs
  (|CallParentFunction OtherActor)
  (Variables|Default|SetActif true)
  (Input|EnableInput (Game|GetPlayerController 0)))

(event EventTick
  (params (DeltaSeconds :type Float%20%28single-precision%29))
  (|CallParentFunction DeltaSeconds))

(event Collision|EventActorEndOverlap
  (params (OtherActor :type Actor%20Object%20Reference))
  ;[0.15 0.15 0.15 0.5] Quand le joueur n'a plus l'objet dans sa main l'objet ne recoit plus ses inputs
  (Variables|Default|SetActif false)
  (Input|DisableInput (Game|GetPlayerController 0) 0))

(fn ConstructionScript
  (|CallParentFunction))