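; Navigation station pickup that snaps onto the raft's "Rudder" socket at BeginPlay and lets a player take the helm.
; PickUp attaches the player to the station, disables movement and adds the IMC_Raft Enhanced Input context through PC_Multi.
; Drop reverses this by detaching, restoring walking and removing the context, with an InUse flag guarding both.
; Overlap and Tick events only forward to the parent class.
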(event OnComponentBeginOverlap(Box)
  (params (OverlappedComponent :type Primitive%20Component%20Object%20Reference) (OtherActor :type Actor%20Object%20Reference) (OtherComp :type Primitive%20Component%20Object%20Reference) (OtherBodyIndex :type Integer) (bFromSweep :type Boolean) (SweepResult :type Hit%20Result%20Structure%20%28by%20ref%29))
  (|CallParentFunction OtherActor))

(event OnComponentEndOverlap(Box)
  (params (OverlappedComponent :type Primitive%20Component%20Object%20Reference) (OtherActor :type Actor%20Object%20Reference) (OtherComp :type Primitive%20Component%20Object%20Reference) (OtherBodyIndex :type Integer))
  (|CallParentFunction OtherActor))

(event EventBeginPlay
  (|CallParentFunction)
  (bind _returnvalue (Actor|GetActorOfClass "/Game/Blueprints/Raft/BP_Raft_Base1.BP_Raft_Base1_C"))
  (Transformation|AttachActorToActor _returnvalue "Rudder" "SnapToTarget" "KeepWorld" "KeepWorld" true))

(event EventTick
  (params (DeltaSeconds :type Float%20%28single-precision%29))
  (|CallParentFunction DeltaSeconds))

(event EventPickUp
  (params (Player :type BP%20Third%20Person%20Character%20Object%20Reference))
  (if (not (Variables|Default|GetinUse?))
    (Transformation|AttachActorToActor (Variables|Default|GetPlayer) self "None" "SnapToTarget" "KeepWorld" "KeepWorld" true)
    (Variables|Default|SetinUse? true)
    (Pawn|Components|CharacterMovement|DisableMovement (Variables|/Script/Engine.Character|GetCharacterMovement (Variables|Default|GetPlayer)))
    (bind _aspc_multi (Utilities|Casting|CastToPC_Multi (Pawn|GetController (Variables|Default|GetPlayer))))
    (Input|AddMappingContext (PlayerController|LocalPlayerSubsystems|GetEnhancedInputLocalPlayerSubsystem _aspc_multi) "/Game/Input/IMC_Raft.IMC_Raft" 1 "(bIgnoreAllPressedKeysUntilRelease=True,bForceImmediately=False,bNotifyUserSettings=False)")))

(event EventDrop
  (params (Player :type BP%20Third%20Person%20Character%20Object%20Reference))
  (if (Variables|Default|GetinUse?)
    (Transformation|DetachFromActor (Variables|Default|GetPlayer) "KeepWorld" "KeepWorld" "KeepWorld")
    (Variables|Default|SetinUse? false)
    (Pawn|Components|CharacterMovement|SetMovementMode (Variables|/Script/Engine.Character|GetCharacterMovement (Variables|Default|GetPlayer)) "MOVE_Walking" 0)
    (bind _aspc_multi (Utilities|Casting|CastToPC_Multi (Pawn|GetController (Variables|Default|GetPlayer))))
    (Input|RemoveMappingContext (PlayerController|LocalPlayerSubsystems|GetEnhancedInputLocalPlayerSubsystem _aspc_multi) "/Game/Input/IMC_Raft.IMC_Raft" "(bIgnoreAllPressedKeysUntilRelease=True,bForceImmediately=False,bNotifyUserSettings=False)")))

(fn ConstructionScript
  (|CallParentFunction))