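; BP_SpawnerPoisson is a fish spawner actor for the fishing station; its graph handles only visual feedback, with no spawning logic.
; SeeFeedback sets the exclamation mark's visibility and plays a timeline that scales it uniformly.
; When the timeline finishes, it plays the WB_Peche joystick animation and shows the widget component, even if the exclamation was set hidden.
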(event Custom|SeeFeedback
  (params (VisibleExclamation :type Boolean))
  (bind _widget (Variables|Default|GetWidget))
  (Rendering|SetVisibility (Variables|Default|GetExclamation) VisibleExclamation false)
  (bind _newtrack_0 (Timeline|ExclamationAnim PlayFromStart)
    (:Update
      (Transformation|SetWorldScale3D (Variables|Default|GetExclamation) (Math|Vector|MakeVector (.x _newtrack_0) (.x _newtrack_0) (.x _newtrack_0))))
    (:Finished
      (bind _aswb_peche (Utilities|Casting|CastToWB_Peche (UserInterface|GetWidget _widget)))
      (UserInterface|Animation|PlayAnimation _aswb_peche (Variables|/Game/Blueprints/Stations/Peche/WB_Peche.WB_Peche_C|GetJoystickAnim _aswb_peche) 0.0 1 "Forward" 1.0 false)
      (Rendering|SetVisibility _widget true false))))

(event EventBeginPlay)

(event Collision|EventActorBeginOverlap
  (params (OtherActor :type Actor%20Object%20Reference)))

(fn ConstructionScript)