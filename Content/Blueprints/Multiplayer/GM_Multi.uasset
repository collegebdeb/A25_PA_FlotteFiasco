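; Game mode for local multiplayer that creates extra players and handles character respawns.
; On BeginPlay it calls CreatePlayer four times, sets the default pawn to BP_ThirdPersonCharacter and restarts the first player.
; The Respawnplayer event spawns a new character at a given transform and has the controller matching the player ID possess it.
; A disconnected player-count snippet is noted as non-working and never runs.
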(event Custom|Respawn%20player
  (params (SpawnTransform :type Transform) (PlayerID :type Integer))
  (bind _returnvalue (Game|SpawnActorfromClass "/Game/ThirdPerson/Blueprints/BP_ThirdPersonCharacter.BP_ThirdPersonCharacter_C" SpawnTransform "Undefined" "MultiplyWithRoot" 0 0))
  (Pawn|Possess (Game|GetPlayerController PlayerID) _returnvalue))

(event EventBeginPlay
  (for _index (range 0 3)
    (Class|GameplayStatics|CreatePlayer -1))
  (Variables|Default|SetDefaultPawnClass "/Game/ThirdPerson/Blueprints/BP_ThirdPersonCharacter.BP_ThirdPersonCharacter_C")
  (Class|GameModeBase|RestartPlayer (Game|GetPlayerController 0)))

(fn ConstructionScript)