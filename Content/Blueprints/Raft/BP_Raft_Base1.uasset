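; Raft base actor that handles falling overboard and spawns breaches on the raft during play.
; Its DeathBox kills overlapping characters and teleports unused fishing rod and harpoon pickups back to RespawnPoint.
; A looping timer, its interval randomized at BeginPlay, spawns capped, raft-attached breaches in three zones, using delayed overlap checks to reposition crowded ones.
; Two functions toggle a custom channel's collision response on characters' held pickups.
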(event OnComponentBeginOverlap(DeathBox)
  (params (OverlappedComponent :type Primitive%20Component%20Object%20Reference) (OtherActor :type Actor%20Object%20Reference) (OtherComp :type Primitive%20Component%20Object%20Reference) (OtherBodyIndex :type Integer) (bFromSweep :type Boolean) (SweepResult :type Hit%20Result%20Structure%20%28by%20ref%29))
  ;[0.15 0.15 0.15 0.5] Death si persos tombent dans l'eau OU si le harpon/canne a peche tombe la respawn sur le radeau
  (Utilities|FlowControl|Sequence
    (:then_0
      (bind _asbp_third_person_character (Utilities|Casting|CastToBP_ThirdPersonCharacter OtherActor))
      (Default|Death _asbp_third_person_character))
    (:then_1
      (bind _asbp_pick_up_pecheur (Utilities|Casting|CastToBP_PickUp_Pecheur OtherActor))
      (if (not (Variables|/Game/Blueprints/Interactable/Parent/BP_Interactable_PickUp.BP_Interactable_PickUp_C|GetinUse? _asbp_pick_up_pecheur))
        (Transformation|SetActorLocation _asbp_pick_up_pecheur (Transformation|GetWorldLocation (Variables|Default|GetRespawnPoint)) false false)))
    (:then_2
      (bind _asbp_pick_up_harpon (Utilities|Casting|CastToBP_PickUp_Harpon OtherActor))
      (if (not (Variables|/Game/Blueprints/Interactable/Parent/BP_Interactable_PickUp.BP_Interactable_PickUp_C|GetinUse? _asbp_pick_up_harpon))
        (Transformation|SetActorLocation _asbp_pick_up_harpon (Transformation|GetWorldLocation (Variables|Default|GetRespawnPoint)) false false)))))

(event Custom|SpawnBreches
  (bind _spawnerbreches1 (Variables|Default|GetSpawnerBreches1))
  (bind _spawnerbreches (Variables|Default|GetSpawnerBreches))
  (bind _spawnerbreches2 (Variables|Default|GetSpawnerBreches2))
  (bind _spawnerbreches1_2 (Variables|Default|GetSpawnerBreches1))
  (bind _spawnerbreches_2 (Variables|Default|GetSpawnerBreches))
  (bind _spawnerbreches2_2 (Variables|Default|GetSpawnerBreches2))
  (bind _array (Utilities|Array|MakeArray _spawnerbreches_2 _spawnerbreches1 _spawnerbreches2_2))
  (bind _array_2 (Utilities|Array|MakeArray _spawnerbreches _spawnerbreches1_2 _spawnerbreches2))
  (bind _outitem (Utilities|Array|Random _array))
  (bind _outitem_2 (Utilities|Array|Random _array_2))
  (bind _returnvalue (Transformation|GetWorldLocation _outitem))
  (bind _returnvalue_2 (Transformation|GetWorldLocation _outitem_2))
  (bind _returnvalue_3 (Math|Random|RandomPointinBoundingBox _returnvalue_2 "100.000000,100.000000,0.000000"))
  (bind _returnvalue_4 (Math|Random|RandomPointinBoundingBox _returnvalue "100.000000,100.000000,0.000000"))
  ;[0.15 0.15 0.15 0.5] Apres un temps predefini, des breches vont spawn. Il y a une limite de breche en jeu
  (for _index (range 0 (Math|Random|RandomIntegerinRange 0 1))
    (if (not (== (Variables|Default|GetNumberOfActors) (Variables|Default|GetMaxActors)))
      (if (not (Variables|Default|GetBrecheTooCloseSpawn?))
        (bind _result (Math|Integer|IncrementInt (Variables|Default|GetNumberOfActors))
          (:%20%20
            (Variables|Default|SetNumberOfActors _result)
            (bind _returnvalue_5 (Game|SpawnActorfromClass "/Game/Blueprints/Stations/Reparation/BP_Breche.BP_Breche_C" (Math|Transform|MakeTransform (Math|Vector|MakeVector (.x _returnvalue_3) (.y _returnvalue_3) 5.0) "0.000000,-180.000000,0.000000" "1.000000,1.000000,1.000000") "Undefined" "MultiplyWithRoot" 0 0))
            (bind _output_get (Variables|Default|SetNewBreche _returnvalue_5))
            (Transformation|AttachComponentToComponent _output_get (Variables|Default|GetSM_Raft) "None" "KeepRelative" "KeepRelative" "KeepRelative" true)
            (Utilities|Array|Add (Variables|Default|GetAllBreches) (Variables|Default|GetNewBreche))
            (for (_array_element _array_index) (Variables|Default|GetAllBreches) :!label _label
              (Utilities|IsValid _array_element
                (:Is%20Valid
                  (bind _outactors (Actor|GetAllActorsOfClass "/Game/Blueprints/Stations/Reparation/BP_Breche.BP_Breche_C"))
                  (Actor|GetActorOfClass "/Game/Blueprints/Stations/Cuisine/BP_PickUp_Cuisine.BP_PickUp_Cuisine_C")
                  (if (or (Collision|IsOverlappingActor _array_element (Utilities|Array|Get(acopy) _outactors _array_index) :!class /Script/Engine.Actor) (Collision|IsOverlappingActor _array_element (Utilities|Array|Get(acopy) _outactors _array_index) :!class /Script/Engine.Actor))
                    (Utilities|FlowControl|Delay 0.01)
                    (Variables|Default|SetBrecheTooCloseSpawn? true)
                    (else
                      (Utilities|FlowControl|Delay 0.01)
                      (Variables|Default|SetBrecheTooCloseSpawn? false))))))
            (Utilities|FlowControl|Delay 0.3)
            (if (Variables|Default|GetBrecheTooCloseSpawn?)
              (Transformation|SetActorLocation _array_element (Math|Vector|MakeVector (.x _returnvalue_4) (.y _returnvalue_4) 5.0) false true)
              (Variables|Default|SetBrecheTooCloseSpawn? false)
              (goto _label))))))))

(event EventBeginPlay
  ;[0.15 0.15 0.15 0.5] Quand le jeu commence et que le rraft est sur la map, ajoute la mini map et commence le timer des breches
  (Utilities|Time|SetTimerbyEvent (delegate Custom|SpawnBreches) (Math|Conversions|ToFloat(Integer) (Math|Random|RandomIntegerinRange (Variables|Default|GetTempsMin) (Variables|Default|GetTempsMax))) true))

(event EventTick
  (params (DeltaSeconds :type Float%20%28single-precision%29))
  (Transformation|SetWorldRotation (Variables|Default|GetRespawnPoint) "0.000000,90.000000,0.000000" false false))

(fn ConstructionScript)

(fn SetCollisionon
  (bind _outactors (Actor|GetAllActorsOfClass "/Game/ThirdPerson/Blueprints/BP_ThirdPersonCharacter.BP_ThirdPersonCharacter_C"))
  (for _array_element _outactors
    (bind _bp_pickup (Variables|/Game/ThirdPerson/Blueprints/BP_ThirdPersonCharacter.BP_ThirdPersonCharacter_C|GetBP_PickUp _array_element)
      (:then
        (Collision|SetCollisionResponsetoChannel (Variables|/Game/Blueprints/Interactable/Parent/BP_Interactable_PickUp.BP_Interactable_PickUp_C|GetSM _bp_pickup) "ECC_GameTraceChannel4" "ECR_Block"))
      (:else))))

(fn SetCollisionOff
  (bind _outactors (Actor|GetAllActorsOfClass "/Game/ThirdPerson/Blueprints/BP_ThirdPersonCharacter.BP_ThirdPersonCharacter_C"))
  (for _array_element _outactors
    (bind _bp_pickup (Variables|/Game/ThirdPerson/Blueprints/BP_ThirdPersonCharacter.BP_ThirdPersonCharacter_C|GetBP_PickUp _array_element)
      (:then
        (Collision|SetCollisionResponsetoChannel (Variables|/Game/Blueprints/Interactable/Parent/BP_Interactable_PickUp.BP_Interactable_PickUp_C|GetSM _bp_pickup) "ECC_GameTraceChannel4" "ECR_Ignore"))
      (:else))))