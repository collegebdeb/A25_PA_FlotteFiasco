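; Cooking station actor that shows a three-step, color-coded seasoning combo from DT_Cook, keyed by Animal, while the player overlaps its box.
; I/J/K/L, enabled at BeginPlay, append directions to Combo, which clears on leaving the box.
; A match with the row's Sequence hides the planes, shows the WB_Cuisine widget and immediately runs Cuisson.
; Cuisson's timing window is disabled, so it resets and hides the widget whenever progress is below 0.99.
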(event OnComponentBeginOverlap(Box)
  (params (OverlappedComponent :type Primitive%20Component%20Object%20Reference) (OtherActor :type Actor%20Object%20Reference) (OtherComp :type Primitive%20Component%20Object%20Reference) (OtherBodyIndex :type Integer) (bFromSweep :type Boolean) (SweepResult :type Hit%20Result%20Structure%20%28by%20ref%29))
  (bind _asbp_third_person_character (Utilities|Casting|CastToBP_ThirdPersonCharacter OtherActor))
  (CallFunction|InputAfficher))

(event OnComponentEndOverlap(Box)
  (params (OverlappedComponent :type Primitive%20Component%20Object%20Reference) (OtherActor :type Actor%20Object%20Reference) (OtherComp :type Primitive%20Component%20Object%20Reference) (OtherBodyIndex :type Integer))
  (Utilities|Casting|CastToBP_ThirdPersonCharacter OtherActor)
  (Rendering|SetVisibility (Variables|Default|GetPlane2) false false)
  (Variables|Default|SetCombo ""))

(event Custom|Cuisson
  ;[0.15 0.15 0.15 0.5] Mini jeu de cuisson
  (bind _aswb_cuisine (Utilities|Casting|CastToWB_Cuisine (UserInterface|GetWidget (Variables|Default|GetWidget))))
  (if (or (Math|Boolean|ANDBoolean (> (Variables|/Script/UMG.ProgressBar|GetPercent (Variables|/Game/Blueprints/CuisineEtPeche/Outils/Cuisine/WB_Cuisine.WB_Cuisine_C|GetProgressBar_0 _aswb_cuisine)) 0.45) (< (Variables|/Script/UMG.ProgressBar|GetPercent (Variables|/Game/Blueprints/CuisineEtPeche/Outils/Cuisine/WB_Cuisine.WB_Cuisine_C|GetProgressBar_0 _aswb_cuisine)) 0.55) false) (< (Variables|/Script/UMG.ProgressBar|GetPercent (Variables|/Game/Blueprints/CuisineEtPeche/Outils/Cuisine/WB_Cuisine.WB_Cuisine_C|GetProgressBar_0 _aswb_cuisine)) 0.99))
    (Default|ResetCuisson _aswb_cuisine)
    (Rendering|SetVisibility (Variables|Default|GetWidget) false false)))

(event Custom|Assaissonement
  (bind _returnvalue (Utilities|GetDataTableRow "/Game/Blueprints/CuisineEtPeche/Outils/Cuisine/DT_Cook.DT_Cook" (Variables|Default|GetAnimal))
    (:then
      (if (Utilities|Enum|Equal(Enum) (.sequence _returnvalue) (Variables|Default|GetCombo))
        (CallFunction|PrepCuisson)))))

(event Custom|InputAfficher
  (bind _plane (Variables|Default|GetPlane))
  (bind _plane1 (Variables|Default|GetPlane1))
  (bind _plane2 (Variables|Default|GetPlane2))
  ;[0.15 0.15 0.15 0.5] Update le combo afficher
  (bind _returnvalue (Utilities|GetDataTableRow "/Game/Blueprints/CuisineEtPeche/Outils/Cuisine/DT_Cook.DT_Cook" (Variables|Default|GetAnimal))
    (:then
      (Rendering|SetVisibility (Variables|Default|GetPlane2) true false)
      (Utilities|FlowControl|Sequence
        (:then_0
          (if (Utilities|Enum|Equal(Enum) (.premierinput _returnvalue) "Up")
            (Rendering|Material|SetMaterial _plane 0 "/Game/Blueprints/CuisineEtPeche/Outils/Mat/M_Vert.M_Vert")
            (elif (Utilities|Enum|Equal(Enum) (.premierinput _returnvalue) "Down")
              (Rendering|Material|SetMaterial _plane 0 "/Game/Blueprints/CuisineEtPeche/Outils/Mat/M_Rouge.M_Rouge")
              (elif (Utilities|Enum|Equal(Enum) (.premierinput _returnvalue) "Left")
                (Rendering|Material|SetMaterial _plane 0 "/Game/Blueprints/CuisineEtPeche/Outils/Mat/M_Jaune.M_Jaune")
                (elif (Utilities|Enum|Equal(Enum) (.premierinput _returnvalue) "Right")
                  (Rendering|Material|SetMaterial _plane 0 "/Game/Blueprints/CuisineEtPeche/Outils/Mat/M_Bleu.M_Bleu")
                  (elif (Utilities|Enum|Equal(Enum) (.premierinput _returnvalue) "")
                    (Rendering|SetVisibility (Variables|Default|GetPlane) false false)))))))
        (:then_1
          (if (Utilities|Enum|Equal(Enum) (.deuxiemeinput _returnvalue) "Up")
            (Rendering|Material|SetMaterial _plane1 0 "/Game/Blueprints/CuisineEtPeche/Outils/Mat/M_Vert.M_Vert")
            (elif (Utilities|Enum|Equal(Enum) (.deuxiemeinput _returnvalue) "Down")
              (Rendering|Material|SetMaterial _plane1 0 "/Game/Blueprints/CuisineEtPeche/Outils/Mat/M_Rouge.M_Rouge")
              (elif (Utilities|Enum|Equal(Enum) (.deuxiemeinput _returnvalue) "Left")
                (Rendering|Material|SetMaterial _plane1 0 "/Game/Blueprints/CuisineEtPeche/Outils/Mat/M_Jaune.M_Jaune")
                (elif (Utilities|Enum|Equal(Enum) (.deuxiemeinput _returnvalue) "Right")
                  (Rendering|Material|SetMaterial _plane1 0 "/Game/Blueprints/CuisineEtPeche/Outils/Mat/M_Bleu.M_Bleu")
                  (elif (Utilities|Enum|Equal(Enum) (.deuxiemeinput _returnvalue) "")
                    (Rendering|SetVisibility (Variables|Default|GetPlane1) false false)))))))
        (:then_2
          (if (Utilities|Enum|Equal(Enum) (.troisiemeinput _returnvalue) "Up")
            (Rendering|Material|SetMaterial _plane2 0 "/Game/Blueprints/CuisineEtPeche/Outils/Mat/M_Vert.M_Vert")
            (elif (Utilities|Enum|Equal(Enum) (.troisiemeinput _returnvalue) "Down")
              (Rendering|Material|SetMaterial _plane2 0 "/Game/Blueprints/CuisineEtPeche/Outils/Mat/M_Rouge.M_Rouge")
              (elif (Utilities|Enum|Equal(Enum) (.troisiemeinput _returnvalue) "Left")
                (Rendering|Material|SetMaterial _plane2 0 "/Game/Blueprints/CuisineEtPeche/Outils/Mat/M_Jaune.M_Jaune")
                (elif (Utilities|Enum|Equal(Enum) (.troisiemeinput _returnvalue) "Right")
                  (Rendering|Material|SetMaterial _plane2 0 "/Game/Blueprints/CuisineEtPeche/Outils/Mat/M_Bleu.M_Bleu")
                  (elif (Utilities|Enum|Equal(Enum) (.troisiemeinput _returnvalue) "")
                    (Rendering|SetVisibility (Variables|Default|GetPlane2) false false)))))))))
    (:RowNotFound
      (Rendering|Material|SetMaterial (Variables|Default|GetPlane2) 0 "/Game/LevelPrototyping/Materials/MI_DefaultColorway.MI_DefaultColorway"))))

(event Custom|PrepCuisson
  (Rendering|SetVisibility (Variables|Default|GetPlane2) false false)
  (Rendering|SetVisibility (Variables|Default|GetWidget) true false)
  (CallFunction|Cuisson))

(event EventTick
  (params (DeltaSeconds :type Float%20%28single-precision%29)))

(event EventBeginPlay
  (Input|EnableInput (Game|GetPlayerController 0)))

(event Input|KeyboardEvents|I
  (params (Key :type Key%20Structure :default "None"))
  (:Pressed
    (Variables|Default|SetCombo (Utilities|String|Append (Variables|Default|GetCombo) "Up"))
    (CallFunction|Assaissonement)))

(event Input|KeyboardEvents|K
  (params (Key :type Key%20Structure :default "None"))
  (:Pressed
    (Variables|Default|SetCombo (Utilities|String|Append (Variables|Default|GetCombo) "Down"))
    (CallFunction|Assaissonement)))

(event Input|KeyboardEvents|J
  (params (Key :type Key%20Structure :default "None"))
  (:Pressed
    (Variables|Default|SetCombo (Utilities|String|Append (Variables|Default|GetCombo) "Left"))
    (CallFunction|Assaissonement)))

(event Input|KeyboardEvents|L
  (params (Key :type Key%20Structure :default "None"))
  (:Pressed
    (Variables|Default|SetCombo (Utilities|String|Append (Variables|Default|GetCombo) "Right"))
    (CallFunction|Assaissonement)))

(fn ConstructionScript)