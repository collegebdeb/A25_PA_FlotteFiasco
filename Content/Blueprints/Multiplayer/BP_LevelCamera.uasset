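; BP_LevelCamera is a level camera that takes over player 0's view on BeginPlay and trails a target actor.
; Each tick, while TargetActor is valid, it eases toward a point behind that actor along its forward vector, scaling the remaining distance by delta time.
; It moves only in X and Y, leaving its height and rotation untouched, and TargetActor is not assigned within this Blueprint.
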(event EventBeginPlay
  (Game|Player|SetViewTargetwithBlend (Game|GetPlayerController 0) self 0.0 "VTBlend_Linear" 0.0 false))

(event EventTick
  (params (DeltaSeconds :type Float%20%28single-precision%29))
  (bind _self self)
  (bind _targetactor (Variables|Default|GetTargetActor))
  (bind _targetactor_2 (Variables|Default|GetTargetActor))
  (bind _returnvalue (Transformation|GetActorForwardVector _targetactor_2))
  (bind _returnvalue_2 (Transformation|GetActorLocation _self))
  (bind _returnvalue_3 (Transformation|GetActorLocation _targetactor))
  (bind _returnvalue_4 (* _returnvalue -1e+03))
  (bind _returnvalue_5 (+ _returnvalue_4 _returnvalue_3))
  (bind _returnvalue_6 (- _returnvalue_5 _returnvalue_2))
  (bind _returnvalue_7 (* DeltaSeconds _returnvalue_6))
  (Variables|Default|GetTargetActor
    (:then
      (Transformation|AddActorWorldOffset (Math|Vector|MakeVector (.x _returnvalue_7) (.y _returnvalue_7) 0.0)))
    (:else)))

(fn ConstructionScript)