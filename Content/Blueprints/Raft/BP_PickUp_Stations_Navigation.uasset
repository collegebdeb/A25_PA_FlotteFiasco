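; Raft navigation station, a pick-up Blueprint that locks the player in place while they navigate.
; PickUp runs the parent logic, snaps the player onto the station, disables their collision and sets IsNavigating.
; Drop detaches the player, restores collision and clears the flag without calling a parent implementation.
; Both events then call ReceivePlayerIndex on the Raft.
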(event EventBeginPlay
  (|CallParentFunction) ; This node is disabled and will not be called.\nDrag off pins to build functionality.
)

(event Collision|EventActorBeginOverlap
  (params (OtherActor :type Actor%20Object%20Reference))
  (|CallParentFunction OtherActor) ; This node is disabled and will not be called.\nDrag off pins to build functionality.
)

(event EventTick
  (params (DeltaSeconds :type Float%20%28single-precision%29))
  (|CallParentFunction DeltaSeconds) ; This node is disabled and will not be called.\nDrag off pins to build functionality.
)

(event EventPickUp
  (params (Player :type BP%20Third%20Person%20Character%20Object%20Reference))
  (|CallParentFunction 0)
  (Transformation|AttachActorToActor (Variables|Default|GetPlayer) self "None" "SnapToTarget" "KeepWorld" "KeepWorld" true)
  (Collision|SetActorEnableCollision (Variables|Default|GetPlayer) false)
  (Variables|Default|SetisNavigating? true)
  (Default|ReceivePlayerIndex (Variables|Default|GetRaft)))

(event EventDrop
  (params (Player :type BP%20Third%20Person%20Character%20Object%20Reference))
  (Transformation|DetachFromActor (Variables|Default|GetPlayer) "KeepWorld" "KeepWorld" "KeepWorld")
  (Collision|SetActorEnableCollision (Variables|Default|GetPlayer) true)
  (Variables|Default|SetisNavigating? false)
  (Default|ReceivePlayerIndex (Variables|Default|GetRaft)))

(fn ConstructionScript
  (|CallParentFunction))