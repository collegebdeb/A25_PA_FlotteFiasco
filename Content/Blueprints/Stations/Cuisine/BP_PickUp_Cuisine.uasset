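; Cooking station pickup on the raft's "Cook" socket where a player holding a fish plays a button-combo minigame.
; Pickup rolls three random inputs from DT_Combo and displays their materials on UI components.
; AddPlayerInput compares entries as they arrive: a mismatch costs energy and rerolls, while a full match boosts energy and drops the item.
; Dropping hides the UI, and leaving the overlap regenerates the combo.
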(event OnComponentEndOverlap(Box)
  (params (OverlappedComponent :type Primitive%20Component%20Object%20Reference) (OtherActor :type Actor%20Object%20Reference) (OtherComp :type Primitive%20Component%20Object%20Reference) (OtherBodyIndex :type Integer))
  ;[0.15 0.15 0.15 0.5] End Overlap - Parent, réinitialise le combo de la station quand le joueur sort.
  (if (Variables|Default|GetisOverlapping?)
    (|CallParentFunction OtherActor)
    (CallFunction|ClearCombo)
    (Variables|Default|SetisOverlapping? false)))

(event Custom|CookingFail
  ;[0.15 0.15 0.15 0.5] Si le mini-jeu échoue, cela génère un nouveau combo aléatoire et inflige une pénalité sur l'énergie.
  (CallFunction|GenerateCombo)
  (CallFunction|EnergyMalusDefeat (Variables|Default|GetEnergyImpact)))

(event Custom|CookingSuccess
  (bind _player (Variables|Default|GetPlayer))
  ;[0.15 0.15 0.15 0.5] Si le mini-jeu réussit, drop l'item et ajoute un boost d'énergie
  (Variables|/Game/ThirdPerson/Blueprints/BP_ThirdPersonCharacter.BP_ThirdPersonCharacter_C|SetPlayerCooking? (Variables|Default|GetPlayer) false)
  (CallFunction|EnergyBoostSuccess (Variables|Default|GetEnergyImpact))
  (Default|DropItem _player self _player)
  (Variables|Default|SetcookingEnCours? false))

(event EventBeginPlay
  ;[0.15 0.15 0.15 0.5] Begin Play - Parent
  (|CallParentFunction)
  (bind _returnvalue (Actor|GetActorOfClass "/Game/Blueprints/Raft/BP_Raft_Base1.BP_Raft_Base1_C"))
  (Transformation|AttachActorToActor _returnvalue "Cook" "SnapToTarget" "KeepWorld" "KeepWorld" true))

(event EventTick
  (params (DeltaSeconds :type Float%20%28single-precision%29))
  ;[0.15 0.15 0.15 0.5] Event Tick - Parent
  (|CallParentFunction DeltaSeconds))

(event EventDrop
  (params (Player :type BP%20Third%20Person%20Character%20Object%20Reference))
  ;[0.15 0.15 0.15 0.5] Event Drop - Parent, désactive le UI de la station et réinitialise les booléens
  (Variables|/Game/ThirdPerson/Blueprints/BP_ThirdPersonCharacter.BP_ThirdPersonCharacter_C|SetPlayerCooking? Player false)
  (|CallParentFunction Player)
  (Rendering|SetVisibility (Variables|Default|GetUI_Combo0) false false)
  (Variables|Default|SetcookingEnCours? false))

(event EventPickUp
  (params (Player :type BP%20Third%20Person%20Character%20Object%20Reference))
  ;[0.15 0.15 0.15 0.5] Quand le joueur prends la station, cela génère un combo aléatoire qui s'affiche à l'écran. Si les input du joueur étaient enregistrés dans le UserCombo, ils sont réinitialisés.
  (if (Variables|/Game/ThirdPerson/Blueprints/BP_ThirdPersonCharacter.BP_ThirdPersonCharacter_C|GethasFish? Player)
    (|CallParentFunction Player)
    (Variables|/Game/ThirdPerson/Blueprints/BP_ThirdPersonCharacter.BP_ThirdPersonCharacter_C|SetPlayerCooking? Player true)
    (if (Utilities|Array|IsEmpty (Variables|Default|GetUserCombo))
      _
      (else
        (Utilities|Array|Clear (Variables|Default|GetUserCombo))))
    (CallFunction|GenerateCombo)
    (Utilities|FlowControl|Delay 0.1)
    (Variables|Default|SetcookingEnCours? true)
    (Rendering|SetVisibility (Variables|Default|GetUI_Combo0) true false)))

(event Collision|EventActorBeginOverlap
  (params (OtherActor :type Actor%20Object%20Reference))
  ;[0.15 0.15 0.15 0.5] Begin Overlap - Parent
  (bind _asbp_third_person_character (Utilities|Casting|CastToBP_ThirdPersonCharacter OtherActor))
  (if (Variables|/Game/ThirdPerson/Blueprints/BP_ThirdPersonCharacter.BP_ThirdPersonCharacter_C|GethasFish? _asbp_third_person_character)
    (|CallParentFunction OtherActor)
    (Variables|Default|SetisOverlapping? true)))

(fn ConstructionScript
  (|CallParentFunction))

(fn GenerateCombo
  ;[0.15 0.15 0.15 0.5] Pour chaque index, on récupère aléatoirement un input de la DataTable. Chaque input est associé à un élément de UI (A,X,Y).
  (for _index (range 0 2)
    (bind _returnvalue (Utilities|GetDataTableRow "/Game/Blueprints/Stations/Cuisine/DT_Combo.DT_Combo" (Utilities|String|StringToName (Utilities|String|ToString(Integer) (Math|Random|RandomIntegerinRange 0 2))))
      (:then
        ;[0.15 0.15 0.15 0.5] Puis je stocke localement les variables aléatoires dans l'array StationCombo et ComboUI afin de les réutiliser plus tard.
        (Utilities|Array|Add (LocalVariables|GetLocalStationCombo) (.Input (Utilities|Struct|BreakS_Combo _returnvalue)))
        (Variables|Default|SetStationCombo (LocalVariables|GetLocalStationCombo))
        (Utilities|Array|Add (LocalVariables|GetLocalUICombo) (.UICombo (Utilities|Struct|BreakS_Combo _returnvalue)))
        (Variables|Default|SetComboUI (LocalVariables|GetLocalUICombo)))))
  (CallFunction|SetUIMaterial))

(fn ClearCombo
  ;[0.15 0.15 0.15 0.5] Réinitalise le combo de la station
  (Utilities|Array|Clear (Variables|Default|GetStationCombo))
  (CallFunction|GenerateCombo))

(fn CompareCombos
  ;[0.15 0.15 0.15 0.5] Pour chaque index du UserCombo, on compare avec chaque index du StationCombo. Si la valeur est égale (input réussit), on passe à l'index suivant, sinon le mini-jeu a échoué et je réinitialise le UserCombo.
  (for (_array_element _array_index) (Variables|Default|GetUserCombo)
    (if (not (== _array_element (Utilities|Array|Get(acopy) (Variables|Default|GetStationCombo) _array_index)))
      (Utilities|Array|Clear (Variables|Default|GetUserCombo))
      (CallFunction|CookingFail)))
  ;[0.15 0.15 0.15 0.5] Permet de continuer la loop jusqu'au dernier index. Si le dernier index du Station combo est le même que le UserCombo et que la loop a été complétée alors le mini-jeu a été réussi et je réinitialise le UserCombo.
  (if (== _array_index (Utilities|Array|LastIndex (Variables|Default|GetStationCombo)))
    (Utilities|Array|Clear (Variables|Default|GetUserCombo))
    (CallFunction|CookingSuccess)))

(fn AddPlayerInput
  (params (UserInput :type Input%20Action%20Object%20Reference))
  ;[0.15 0.15 0.15 0.5] Fonction qui communique avec le joueur afin de récupérer ses inputs et les stocker dans l'array UserCombo puis comparer avec le StationCombo (fonction Compare)
  (if (Variables|Default|GetcookingEnCours?)
    (Utilities|Array|Add (Variables|Default|GetUserCombo) UserInput)
    (CallFunction|CompareCombos)))

(fn SetUIMaterial
  ;[0.15 0.15 0.15 0.5] Mets à jour le UI en fonction du combo de la station.
  (Rendering|Material|SetMaterial (Variables|Default|GetUI_Combo0) 0 (Utilities|Array|Get(acopy) (Variables|Default|GetComboUI)))
  (Rendering|Material|SetMaterial (Variables|Default|GetUI_Combo1) 0 (Utilities|Array|Get(acopy) (Variables|Default|GetComboUI) 1))
  (Rendering|Material|SetMaterial (Variables|Default|GetUI_Combo2) 0 (Utilities|Array|Get(acopy) (Variables|Default|GetComboUI) 2)))