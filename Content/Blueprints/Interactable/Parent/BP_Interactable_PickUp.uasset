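; Base pickup Blueprint for raft multiplayer: players carry and drop physics items that can affect energy.
; DT_Pickup rows, keyed by PickupType, supply mapping context, energy impact and attach socket.
; Overlap shows a player-colored outline and prompt; fish carriers only get it on BP_PickUp_Cuisine.
; PickUp attaches to the player's mesh, adds the input context and disables item and raft collision; Drop reverses this.
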(event EventPickUp
  (params (Player :type BP%20Third%20Person%20Character%20Object%20Reference))
  ;[0.15 0.15 0.15 0.5] Pick Up - Attache le interactable/collectible au joueur et communique avec le Blueprint du joueur.
  (if (not (and (Variables|Default|GetinUse?) (Variables|/Game/ThirdPerson/Blueprints/BP_ThirdPersonCharacter.BP_ThirdPersonCharacter_C|GetisItemHolded? Player)))
    (bind _output_get (Variables|Default|SetPlayer Player))
    (CallFunction|AddMappingContext _output_get)
    (Variables|Default|SetinUse? true)
    (bind _returnvalue (Utilities|GetDataTableRow "/Game/Blueprints/Interactable/Parent/DT_Pickup.DT_Pickup" (Utilities|String|StringToName (Utilities|String|EnumtoString (Variables|Default|GetPickup_type))))
      (:then
        (Transformation|AttachComponentToComponent (Variables|/Script/Engine.Character|GetMesh (Variables|Default|GetPlayer)) (.SocketName (Utilities|Struct|BreakS_Pickup _returnvalue)) "SnapToTarget" "SnapToTarget" "KeepWorld" true)
        (Default|SetPickupType (Variables|Default|GetPlayer) (Variables|Default|GetPickup_type) self)
        (Audio|PlaySound2D "/Game/Sounds/SFX/ButtonUI.ButtonUI" 1.0 1.0 0.0 0 0)
        (Default|SetCollisionOff (Variables|Default|GetRaft))
        (CallFunction|SetCollisionOff)
        (CallFunction|DisableOverlapFeedback)
        (Variables|Default|SetCurrentPlayerIndex (Class|GameplayStatics|GetPlayerControllerID (.AsPC%20Multi (Utilities|Casting|CastToPC_Multi (Pawn|GetController (Variables|Default|GetPlayer))))))))))

(event Collision|EventActorBeginOverlap
  (params (OtherActor :type Actor%20Object%20Reference))
  (bind _self self)
  ;[0.15 0.15 0.15 0.5] Begin Overlap - Affiche un outliner de la couleur du joueur + le widget A
  (if (not (Variables|Default|GetinUse?))
    (bind _asbp_third_person_character (Utilities|Casting|CastToBP_ThirdPersonCharacter OtherActor))
    (if (Variables|/Game/ThirdPerson/Blueprints/BP_ThirdPersonCharacter.BP_ThirdPersonCharacter_C|GetisItemHolded? _asbp_third_person_character)
      (if (Variables|/Game/ThirdPerson/Blueprints/BP_ThirdPersonCharacter.BP_ThirdPersonCharacter_C|GethasFish? _asbp_third_person_character)
        (if (== (Utilities|GetClass _self) "/Game/Blueprints/Stations/Cuisine/BP_PickUp_Cuisine.BP_PickUp_Cuisine_C")
          (Variables|Default|SetCurrentPickUp _self)
          (Variables|Default|SetAs%20BP%20Interactable%20Pick%20Up _self)
          ;;[0 0.2623 0.3564 0.502] Affichage du feedback visuel
          (if (not (Variables|BP_Interactable_PickUp_C|GetinUse? (Variables|Default|GetAs%20BP%20Interactable%20Pick%20Up))) :!label _label
            (Utilities|FlowControl|Sequence
              (:then_0
                (bind _aspc_multi (Utilities|Casting|CastToPC_Multi (Pawn|GetController _asbp_third_person_character)))
                (Rendering|Material|SetOverlayMaterial (Variables|BP_Interactable_PickUp_C|GetSM (Variables|Default|GetAs%20BP%20Interactable%20Pick%20Up)) (Utilities|Array|Get(acopy) (Variables|Default|GetOutlinerColors) (Class|GameplayStatics|GetPlayerControllerID _aspc_multi)) :!class /Script/Engine.MeshComponent))
              (:then_1
                (if (not (Rendering|IsVisible (Variables|BP_Interactable_PickUp_C|GetWidgetA (Variables|Default|GetAs%20BP%20Interactable%20Pick%20Up))))
                  (Rendering|SetVisibility (Variables|BP_Interactable_PickUp_C|GetWidgetA (Variables|Default|GetAs%20BP%20Interactable%20Pick%20Up)) true false)))))))
      (else
        (bind _output_get (Variables|Default|SetCurrentPickUp (Utilities|Array|Get(acopy) (Collision|GetOverlappingActors (Variables|/Script/Engine.Character|GetCapsuleComponent _asbp_third_person_character) "BP_Interactable_PickUp_C" :!class /Script/Engine.PrimitiveComponent))))
        (bind _asbp_interactable_pick_up (Utilities|Casting|CastToBP_Interactable_PickUp _output_get))
        (if (!= (Utilities|GetClass _asbp_interactable_pick_up) "/Game/Blueprints/Stations/Cuisine/BP_PickUp_Cuisine.BP_PickUp_Cuisine_C")
          (Variables|Default|SetAs%20BP%20Interactable%20Pick%20Up _asbp_interactable_pick_up)
          (goto _label))))))

(event EventTick
  (params (DeltaSeconds :type Float%20%28single-precision%29))
  ;[0.15 0.15 0.15 0.5] Event Tick
  (if (Variables|Default|GetinUse?)
    (Development|PrintString (Utilities|String|ToString(Integer) (Variables|Default|GetCurrentPlayerIndex)) true true "(R=0.000000,G=0.660000,B=1.000000,A=1.000000)" 0.0)))

(event EventDrop
  (params (Player :type BP%20Third%20Person%20Character%20Object%20Reference))
  ;[0.15 0.15 0.15 0.5] Drop - Détache le collectible/interactable du joueur et réactive sa physique.
  (if (Variables|Default|GetinUse?)
    (Transformation|DetachFromActor "KeepWorld" "KeepWorld" "KeepWorld")
    (Variables|Default|SetinUse? false)
    (Default|SetCollisionon (Variables|Default|GetRaft))
    (CallFunction|SetCollisionon)
    (CallFunction|RemoveMappingContext Player)
    (Variables|Default|SetPlayer 0)))

(event Collision|EventActorEndOverlap
  (params (OtherActor :type Actor%20Object%20Reference))
  ;[0.15 0.15 0.15 0.5] End Overlap - Désactive le feedback visuel
  (Utilities|Casting|CastToBP_ThirdPersonCharacter OtherActor)
  ;;[0 0.2623 0.3564 0.502] Désactive feedback visuel
  (Rendering|Material|SetOverlayMaterial (Variables|Default|GetSM) 0 :!class /Script/Engine.MeshComponent)
  (if (not (Variables|Default|GetinUse?))
    (bind _asbp_interactable_pick_up (Utilities|Casting|CastToBP_Interactable_PickUp (Variables|Default|GetCurrentPickUp)))
    (Utilities|FlowControl|Sequence
      (:then_0
        (Variables|Default|GetPlayer
          (:then
            (Variables|Default|SetPlayer 0))
          (:else)))
      (:then_1
        (if (Rendering|IsVisible (Variables|BP_Interactable_PickUp_C|GetWidgetA _asbp_interactable_pick_up))
          (Rendering|SetVisibility (Variables|BP_Interactable_PickUp_C|GetWidgetA _asbp_interactable_pick_up) false false))))))

(event EventBeginPlay
  ;[0.15 0.15 0.15 0.5] Begin Play - Récupère certaines valeurs de la DataTable pour les assigner aux pickups.
  (Class|PrimitiveComponent|SetMassOverrideinKg (Variables|Default|GetSM) "None" 0.001 true)
  (bind _returnvalue (Utilities|GetDataTableRow "/Game/Blueprints/Interactable/Parent/DT_Pickup.DT_Pickup" (Utilities|String|StringToName (Utilities|String|EnumtoString (Variables|Default|GetPickup_type))))
    (:then
      (Variables|Default|SetMappingContext (.MappingContext (Utilities|Struct|BreakS_Pickup _returnvalue)))
      (Variables|Default|SetEnergyImpact (.EnergyImpact (Utilities|Struct|BreakS_Pickup _returnvalue)))
      (bind _returnvalue_2 (Actor|GetActorOfClass "/Game/Blueprints/Raft/BP_Raft_Base1.BP_Raft_Base1_C"))
      (Variables|Default|SetRaft _returnvalue_2))))

(fn ConstructionScript
  (Physics|SetSimulatePhysics (Variables|Default|GetSM) true)
  (Components|StaticMesh|SetStaticMesh (Variables|Default|GetSM) (Variables|Default|GetPickup%20SM))
  (Class|PrimitiveComponent|SetMassOverrideinKg (Variables|Default|GetSM) "None" 0.001 true)
  (bind _returnvalue (Utilities|GetDataTableRow "/Game/Blueprints/Interactable/Parent/DT_Pickup.DT_Pickup" (Utilities|String|StringToName (Utilities|String|EnumtoString (Variables|Default|GetPickup_type))))
    (:then
      (Variables|Default|SetEnergyImpact (.EnergyImpact (Utilities|Struct|BreakS_Pickup _returnvalue)))
      (bind _returnvalue_2 (Actor|GetActorOfClass "/Game/Blueprints/Raft/BP_Raft_Base1.BP_Raft_Base1_C"))
      (Variables|Default|SetRaft _returnvalue_2))))

(fn EnergyBoostSuccess
  (params (EnergyImpact :type Float%20%28double-precision%29) (Player%20Index :type Integer))
  (bind _asgm_multi (Utilities|Casting|CastToGM_Multi (Game|GetGameMode)))
  (Default|AddEnergy (Variables|/Game/Blueprints/Multiplayer/GM_Multi.GM_Multi_C|GetWB_Energy _asgm_multi) EnergyImpact (Variables|Default|GetCurrentPlayerIndex))
  (Development|PrintString "add energy" true true "(R=0.000000,G=0.768000,B=0.195030,A=1.000000)" 1e+02))

(fn EnergyMalusDefeat
  (params (EnergyImpact :type Float%20%28double-precision%29))
  (bind _asgm_multi (Utilities|Casting|CastToGM_Multi (Game|GetGameMode)))
  (Default|RemoveEnergy (Variables|/Game/Blueprints/Multiplayer/GM_Multi.GM_Multi_C|GetWB_Energy _asgm_multi) EnergyImpact)
  (Development|PrintString "remove energy" true true "(R=0.000000,G=0.768000,B=0.195030,A=1.000000)" 1e+02))

(fn SetCollisionOff
  (Class|PrimitiveComponent|SetMassOverrideinKg (Variables|Default|GetSM) "None" 0.0001 true)
  (Physics|SetSimulatePhysics (Variables|Default|GetSM) false)
  (Collision|SetCollisionResponsetoChannel (Variables|Default|GetSM) "ECC_WorldStatic" "ECR_Ignore")
  (Collision|SetCollisionResponsetoChannel (Variables|Default|GetSM) "ECC_WorldDynamic" "ECR_Ignore")
  (Collision|SetCollisionResponsetoChannel (Variables|Default|GetSM) "ECC_Visibility" "ECR_Ignore")
  (Collision|SetCollisionResponsetoChannel (Variables|Default|GetSM) "ECC_PhysicsBody" "ECR_Ignore")
  (Collision|SetCollisionResponsetoChannel (Variables|Default|GetSM) "ECC_GameTraceChannel1" "ECR_Ignore")
  (Collision|SetCollisionResponsetoChannel (Variables|Default|GetSM) "ECC_GameTraceChannel2" "ECR_Ignore")
  (Collision|SetCollisionResponsetoChannel (Variables|Default|GetSM) "ECC_GameTraceChannel4" "ECR_Ignore"))

(fn SetCollisionon
  (Physics|SetSimulatePhysics (Variables|Default|GetSM) true)
  (Collision|SetCollisionResponsetoChannel (Variables|Default|GetSM) "ECC_WorldStatic" "ECR_Overlap")
  (Collision|SetCollisionResponsetoChannel (Variables|Default|GetSM) "ECC_WorldDynamic" "ECR_Overlap")
  (Collision|SetCollisionResponsetoChannel (Variables|Default|GetSM) "ECC_Visibility" "ECR_Overlap")
  (Collision|SetCollisionResponsetoChannel (Variables|Default|GetSM) "ECC_PhysicsBody" "ECR_Block")
  (Collision|SetCollisionResponsetoChannel (Variables|Default|GetSM) "ECC_GameTraceChannel1" "ECR_Block")
  (Collision|SetCollisionResponsetoChannel (Variables|Default|GetSM) "ECC_GameTraceChannel2" "ECR_Block")
  (Collision|SetCollisionResponsetoChannel (Variables|Default|GetSM) "ECC_GameTraceChannel4" "ECR_Block"))

(fn AddPlayerinArray
  (params (Object :type Object%20Object%20Reference))
  (bind _playersarray (Variables|Default|GetPlayersArray))
  (bind _output (Utilities|Array|Get(acopy) _playersarray))
  (bind _returnvalue (Pawn|GetController _output))
  (bind _asbp_third_person_character (Utilities|Casting|CastToBP_ThirdPersonCharacter Object))
  (if (not (Utilities|Array|ContainsItem (Variables|Default|GetPlayersArray) _asbp_third_person_character))
    (Utilities|Array|Add (Variables|Default|GetPlayersArray) _asbp_third_person_character)
    (bind _output_get (Variables|Default|SetPlayer (Utilities|Array|Get(acopy) (Variables|Default|GetPlayersArray))))
    (Utilities|IsValid _output_get
      (:Is%20Valid
        (Default|SetPickupType _output_get (Variables|Default|GetPickup_type) self)
        (Variables|Default|SetCurrentPlayerController _returnvalue)
        (bind _aspc_multi (Utilities|Casting|CastToPC_Multi _returnvalue))
        (Rendering|Material|SetOverlayMaterial (Variables|Default|GetSM) (Utilities|Array|Get(acopy) (Variables|Default|GetOutlinerColors) (Class|GameplayStatics|GetPlayerControllerID _aspc_multi)) :!class /Script/Engine.MeshComponent)))))

(fn RemovePlayerinArray
  (params (Object :type Object%20Object%20Reference))
  (bind _playersarray (Variables|Default|GetPlayersArray))
  (bind _output (Utilities|Array|Get(acopy) _playersarray))
  (bind _asbp_third_person_character (Utilities|Casting|CastToBP_ThirdPersonCharacter Object))
  (if (Utilities|Array|ContainsItem (Variables|Default|GetPlayersArray) _asbp_third_person_character)
    (Utilities|Array|RemoveItem (Variables|Default|GetPlayersArray) _asbp_third_person_character)
    (Utilities|IsValid _output
      (:Is%20Valid
        (Variables|Default|SetCurrentPlayerController (Pawn|GetController _output))))))

(fn AddMappingContext
  (params (Player :type BP%20Third%20Person%20Character%20Object%20Reference))
  (Utilities|IsValid (Variables|Default|GetMappingContext)
    (:Is%20Valid
      (bind _aspc_multi (Utilities|Casting|CastToPC_Multi (Pawn|GetController Player)))
      (Input|AddMappingContext (PlayerController|LocalPlayerSubsystems|GetEnhancedInputLocalPlayerSubsystem _aspc_multi) (Variables|Default|GetMappingContext) 1 "(bIgnoreAllPressedKeysUntilRelease=True,bForceImmediately=False,bNotifyUserSettings=False)"))))

(fn RemoveMappingContext
  (params (Player :type BP%20Third%20Person%20Character%20Object%20Reference))
  (Utilities|IsValid (Variables|Default|GetMappingContext)
    (:Is%20Valid
      (bind _aspc_multi (Utilities|Casting|CastToPC_Multi (Pawn|GetController Player)))
      (Input|RemoveMappingContext (PlayerController|LocalPlayerSubsystems|GetEnhancedInputLocalPlayerSubsystem _aspc_multi) (Variables|Default|GetMappingContext) "(bIgnoreAllPressedKeysUntilRelease=True,bForceImmediately=False,bNotifyUserSettings=False)"))))

(fn DisableOverlapFeedback
  (bind _asbp_interactable_pick_up (Utilities|Casting|CastToBP_Interactable_PickUp (Variables|Default|GetCurrentPickUp)))
  (Utilities|FlowControl|Sequence
    (:then_0
      (Rendering|Material|SetOverlayMaterial (Variables|BP_Interactable_PickUp_C|GetSM _asbp_interactable_pick_up) 0 :!class /Script/Engine.MeshComponent))
    (:then_1
      (if (Rendering|IsVisible (Variables|BP_Interactable_PickUp_C|GetWidgetA _asbp_interactable_pick_up))
        (Rendering|SetVisibility (Variables|BP_Interactable_PickUp_C|GetWidgetA _asbp_interactable_pick_up) false false)))))