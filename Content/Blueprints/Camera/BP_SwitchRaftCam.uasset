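; BP_SwitchRaftCam is a trigger volume that rotates the level camera when the raft enters it.
; BeginPlay finds the level camera and raft and caches the camera's starting rotation.
; Overlap by the raft mesh opens a timed window where Tick interpolates the camera toward the Arrow's rotation, with TransitionSpeed serving as both duration and interp speed.
; Outside that window, ResetToOriginalRotation makes Tick snap the camera back every frame.
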(event OnComponentBeginOverlap(Box)
  (params (OverlappedComponent :type Primitive%20Component%20Object%20Reference) (OtherActor :type Actor%20Object%20Reference) (OtherComp :type Primitive%20Component%20Object%20Reference) (OtherBodyIndex :type Integer) (bFromSweep :type Boolean) (SweepResult :type Hit%20Result%20Structure%20%28by%20ref%29))
  (if (== OtherComp (Variables|/Game/Blueprints/Raft/BP_Raft_Base1.BP_Raft_Base1_C|GetSM_Raft (Variables|Default|GetBP_Raft)))
    (Variables|Default|SetRaftHit true)
    (Utilities|FlowControl|Delay (Variables|Default|GetTransitionSpeed))
    (Variables|Default|SetRaftHit false)))

(event EventBeginPlay
  (bind _returnvalue (Actor|GetActorOfClass "/Game/Blueprints/Camera/BP_LevelCamera.BP_LevelCamera_C"))
  (bind _output_get (Variables|Default|SetRaftCam _returnvalue))
  (Variables|Default|SetRaftCamOriginalRotation (Transformation|GetActorRotation _output_get))
  (bind _returnvalue_2 (Actor|GetActorOfClass "/Game/Blueprints/Raft/BP_Raft_Base1.BP_Raft_Base1_C"))
  (Variables|Default|SetBP_Raft _returnvalue_2))

(event EventTick
  (params (DeltaSeconds :type Float%20%28single-precision%29))
  (bind _raftcam (Variables|Default|GetRaftCam))
  (if (Variables|Default|GetRaftHit)
    (Transformation|SetActorRotation _raftcam (Math|Interpolation|RInterpTo (Transformation|GetActorRotation _raftcam) (Transformation|GetWorldRotation (Variables|Default|GetArrow)) DeltaSeconds (Variables|Default|GetTransitionSpeed)))
    (elif (Variables|Default|GetResetToOriginalRotation)
      (Transformation|SetActorRotation (Variables|Default|GetRaftCam) (Variables|Default|GetRaftCamOriginalRotation)))))

(fn ConstructionScript)