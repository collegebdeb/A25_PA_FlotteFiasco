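; Collectible fish for the fishing station that can despawn on a timer after it spawns.
; SetTimerAfterSpawn starts the despawn timer; when it fires, the fish destroys itself unless PickUpPeche reports fishing in progress, in which case the timer is cleared.
; The construction script finds BP_PickUp_Pecheur by class for that check.
; On destruction, the fish tells BPRandomSPawner to remove it from the actor count.
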(event Custom|DestroySpawnedPoisson
  ;[0.15 0.15 0.15 0.5] Fonction qui détruit le poisson après avoir été spawn si le timer est fini si la pêche est pas en cours
  (if (Variables|/Game/Blueprints/Stations/Peche/BP_PickUp_Pecheur.BP_PickUp_Pecheur_C|GetPecheEnCours (Variables|Default|GetPickUp%20Peche))
    (CallFunction|StopTimerDestroySpawned)
    (else
      (Actor|DestroyActor))))

(event Custom|SetTimerAfterSpawn
  ;[0.15 0.15 0.15 0.5] Lance un timer qui va détruire le poisson après avoir été spawn
  (bind _returnvalue (Utilities|Time|SetTimerbyEvent (delegate Custom|DestroySpawnedPoisson) (Variables|Default|GetTempsDespawnPoissons))))

(event Custom|StopTimerDestroySpawned
  ;[0.15 0.15 0.15 0.5] Arrête le timer pour détruire après spawn
  (Utilities|Time|ClearandInvalidateTimerbyHandle (stale Custom|SetTimerAfterSpawn _returnvalue)))

(event EventDestroyed
  (Default|RemovefromNumberofActors (Variables|Default|GetBP_RandomSPawner)))

(fn ConstructionScript
  (bind _returnvalue (Actor|GetActorOfClass "/Game/Blueprints/Stations/Peche/BP_PickUp_Pecheur.BP_PickUp_Pecheur_C"))
  (Variables|Default|SetPickUp%20Peche _returnvalue))