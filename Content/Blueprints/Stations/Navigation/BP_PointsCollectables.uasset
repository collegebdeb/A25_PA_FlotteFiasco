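; BP_PointsCollectables is a pickup actor that awards score when the raft reaches it while the navigation station is manned.
; On BeginPlay it caches the first raft and navigation station actors found in the level.
; When its Box overlaps the raft mesh and the station is in use, it adds its PlayerScoreImpact to that station's player as a non-malus score, then destroys itself.
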(event OnComponentBeginOverlap(Box)
  (params (OverlappedComponent :type Primitive%20Component%20Object%20Reference) (OtherActor :type Actor%20Object%20Reference) (OtherComp :type Primitive%20Component%20Object%20Reference) (OtherBodyIndex :type Integer) (bFromSweep :type Boolean) (SweepResult :type Hit%20Result%20Structure%20%28by%20ref%29))
  (bind _stationnavigateur (Variables|Default|GetStationNavigateur))
  (if (== OtherComp (Variables|/Game/Blueprints/Raft/BP_Raft_Base1.BP_Raft_Base1_C|GetSM_Raft (Variables|Default|GetRaft)))
    (if (Variables|/Game/Blueprints/Interactable/Parent/BP_Interactable_PickUp.BP_Interactable_PickUp_C|GetinUse? _stationnavigateur)
      (Default|UpdateScore (Variables|/Game/Blueprints/Interactable/Parent/BP_Interactable_PickUp.BP_Interactable_PickUp_C|GetPlayer _stationnavigateur) (Variables|Default|GetPlayer%20Score%20Impact) false)
      (Actor|DestroyActor))))

(event EventBeginPlay
  (bind _returnvalue (Actor|GetActorOfClass "/Game/Blueprints/Raft/BP_Raft_Base1.BP_Raft_Base1_C"))
  (Variables|Default|SetRaft _returnvalue)
  (bind _returnvalue_2 (Actor|GetActorOfClass "/Game/Blueprints/Stations/Navigation/BP_PickUp_Stations_Navigation.BP_PickUp_Stations_Navigation_C"))
  (Variables|Default|SetStationNavigateur _returnvalue_2))

(event EventTick
  (params (DeltaSeconds :type Float%20%28single-precision%29)))

(fn ConstructionScript)